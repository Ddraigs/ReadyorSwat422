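; Character creation preview actor that shows the player's chosen looks on a skeletal mesh.
; The construction script puts a dynamic instance of the MBlab human skin material on the mesh.
; From BeginPlay, a looping timer polls the looks stored in RoSGameInstance and applies them to male face and head morph targets and the skin's base colour multiplier.
; Each update also prints debug text, and the VisualUpdate function is empty.
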(event Custom|Update|Target1
  (bind _skeletalmesh (Variables|Default|GetSkeletalMesh))
  (bind _gameinstance (Variables|Default|GetGameInstance))
  (bind _gameinstance_2 (Variables|Default|GetGameInstance))
  (bind _gameinstance_3 (Variables|Default|GetGameInstance))
  (bind _floatvalue (Default|GetLooks _gameinstance_2 "NewEnumerator1"))
  (Development|PrintString "UpdatedMEsh")
  (Development|PrintString (Utilities|String|ToString(Float) _floatvalue))
  (Components|SkeletalMesh|SetMorphTarget _skeletalmesh "MaleHeadShape1" _floatvalue true)
  (Components|SkeletalMesh|SetMorphTarget _skeletalmesh "MaleHeadShape2" (.FloatValue (Default|GetLooks _gameinstance_2 "NewEnumerator2")) true)
  (Components|SkeletalMesh|SetMorphTarget _skeletalmesh "MaleHeadShape3" (.FloatValue (Default|GetLooks _gameinstance_2 "NewEnumerator3")) true)
  (Components|SkeletalMesh|SetMorphTarget _skeletalmesh "MaleBackHeadShape1" (.FloatValue (Default|GetLooks _gameinstance_3 "NewEnumerator5")) true)
  (Components|SkeletalMesh|SetMorphTarget _skeletalmesh "MaleEyeSize" (.FloatValue (Default|GetLooks _gameinstance_3 "NewEnumerator6")) true)
  (Components|SkeletalMesh|SetMorphTarget _skeletalmesh "MaleEyeType1" (.FloatValue (Default|GetLooks _gameinstance_3 "NewEnumerator7")) true)
  (Components|SkeletalMesh|SetMorphTarget _skeletalmesh "MaleEyeTyp2" (.FloatValue (Default|GetLooks _gameinstance "NewEnumerator8")) true)
  (Components|SkeletalMesh|SetMorphTarget _skeletalmesh "MaleEyeSinus" (.FloatValue (Default|GetLooks _gameinstance "NewEnumerator9")) true)
  (Components|SkeletalMesh|SetMorphTarget _skeletalmesh "MaleMouthSize" (.FloatValue (Default|GetLooks _gameinstance "NewEnumerator10")) true)
  (Components|SkeletalMesh|SetMorphTarget _skeletalmesh "MaleLipVolume" (.FloatValue (Default|GetLooks _gameinstance "NewEnumerator11")) true)
  (Rendering|Material|SetVectorParameterValue (Variables|Default|GetDynamicMat) "BaseColourMulti" (Math|Conversions|ToLinearColor(Color) (.Colour (Default|GetLooks _gameinstance "NewEnumerator13"))) :!class /Script/Engine.MaterialInstanceDynamic))

(event EventBeginPlay
  (bind _asro_sgame_instance (Utilities|Casting|CastToRoSGameInstance (Game|GetGameInstance)))
  (Variables|Default|SetGameInstance _asro_sgame_instance)
  (Utilities|Time|SetTimerbyEvent (delegate Custom|Update|Target1) 0.4 true))

(event Collision|EventActorBeginOverlap
  (params (OtherActor :type Actor%20Object%20Reference)))

(event EventTick
  (params (DeltaSeconds :type Float%20%28single-precision%29)))

(fn ConstructionScript
  (bind _returnvalue (Rendering|Material|CreateDynamicMaterialInstance "/Game/ReadyOrSwat/BluePrint/CharCreation/Meshs/MBlab_human_skin_Inst.MBlab_human_skin_Inst" "None" :!class /Script/Engine.KismetMaterialLibrary))
  (bind _output_get (Variables|Default|SetDynamicMat _returnvalue))
  (Rendering|Material|SetMaterial (Variables|Default|GetSkeletalMesh) 0 _output_get))

(fn VisualUpdate)
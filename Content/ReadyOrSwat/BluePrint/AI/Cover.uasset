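; Two-sided cover actor, with a mesh set in construction, that tells overlapping actors implementing CoverInterface when cover is available.
; Each side's volume sends availability and its arrow's rotation and updates Taken, while left and right edge boxes report cover ends.
; Edge exits test the interface on the overlapped component instead of the other actor.
; A looping timer clears Taken when the stored actor reference is invalid.
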(event OnComponentBeginOverlap(Cover1)
  (params (OverlappedComponent :type Primitive%20Component%20Object%20Reference) (OtherActor :type Actor%20Object%20Reference) (OtherComp :type Primitive%20Component%20Object%20Reference) (OtherBodyIndex :type Integer) (bFromSweep :type Boolean) (SweepResult :type Hit%20Result%20Structure%20%28by%20ref%29))
  ;[1 1 1] TakeCOver_1
  (Variables|Default|SetActorRef OtherActor)
  (if (Utilities|DoesObjectImplementInterface OtherActor (Variables|Default|GetCoverInterface))
    (Class|CoverInterface|IsCoverAvilable(Message) OtherActor true (Transformation|GetWorldRotation (Variables|Default|GetArrow)))
    (Variables|Default|SetTaken true)))

(event OnComponentEndOverlap(Cover1)
  (params (OverlappedComponent :type Primitive%20Component%20Object%20Reference) (OtherActor :type Actor%20Object%20Reference) (OtherComp :type Primitive%20Component%20Object%20Reference) (OtherBodyIndex :type Integer))
  ;[1 1 1] TakeCOver_1
  (if (Utilities|DoesObjectImplementInterface OtherActor (Variables|Default|GetCoverInterface))
    (Class|CoverInterface|IsCoverAvilable(Message) OtherActor false "0, 0, 0")
    (Variables|Default|SetTaken false)
    (Variables|Default|SetActorRef 0)))

(event OnComponentEndOverlap(BoxEndOfCover1_Right)
  (params (OverlappedComponent :type Primitive%20Component%20Object%20Reference) (OtherActor :type Actor%20Object%20Reference) (OtherComp :type Primitive%20Component%20Object%20Reference) (OtherBodyIndex :type Integer))
  (if (Utilities|DoesObjectImplementInterface OverlappedComponent (Variables|Default|GetCoverInterface))
    (Class|CoverInterface|EndOfCover(Message) OtherActor false false)
    (Variables|Default|SetTaken false)))

(event OnComponentBeginOverlap(Cover2)
  (params (OverlappedComponent :type Primitive%20Component%20Object%20Reference) (OtherActor :type Actor%20Object%20Reference) (OtherComp :type Primitive%20Component%20Object%20Reference) (OtherBodyIndex :type Integer) (bFromSweep :type Boolean) (SweepResult :type Hit%20Result%20Structure%20%28by%20ref%29))
  ;[1 1 1] TakeCover 2
  (Variables|Default|SetActorRef OtherActor)
  (if (Utilities|DoesObjectImplementInterface OtherActor (Variables|Default|GetCoverInterface))
    (Class|CoverInterface|IsCoverAvilable(Message) OtherActor true (Transformation|GetWorldRotation (Variables|Default|GetArrow1)))
    (Variables|Default|SetTaken true)))

(event OnComponentEndOverlap(Cover2)
  (params (OverlappedComponent :type Primitive%20Component%20Object%20Reference) (OtherActor :type Actor%20Object%20Reference) (OtherComp :type Primitive%20Component%20Object%20Reference) (OtherBodyIndex :type Integer))
  ;[1 1 1] TakeCover 2
  (if (Utilities|DoesObjectImplementInterface OtherActor (Variables|Default|GetCoverInterface))
    (Class|CoverInterface|IsCoverAvilable(Message) OtherActor false "0, 0, 0")
    (Variables|Default|SetTaken false)
    (Variables|Default|SetActorRef 0)))

(event OnComponentBeginOverlap(BoxEndOfCover2_Right)
  (params (OverlappedComponent :type Primitive%20Component%20Object%20Reference) (OtherActor :type Actor%20Object%20Reference) (OtherComp :type Primitive%20Component%20Object%20Reference) (OtherBodyIndex :type Integer) (bFromSweep :type Boolean) (SweepResult :type Hit%20Result%20Structure%20%28by%20ref%29))
  (if (Utilities|DoesObjectImplementInterface OtherActor (Variables|Default|GetCoverInterface))
    (Class|CoverInterface|EndOfCover(Message) OtherActor false true)))

(event OnComponentEndOverlap(BoxEndOfCover2_Left)
  (params (OverlappedComponent :type Primitive%20Component%20Object%20Reference) (OtherActor :type Actor%20Object%20Reference) (OtherComp :type Primitive%20Component%20Object%20Reference) (OtherBodyIndex :type Integer))
  (if (Utilities|DoesObjectImplementInterface OverlappedComponent (Variables|Default|GetCoverInterface))
    (Class|CoverInterface|EndOfCover(Message) OtherActor false false)
    (Variables|Default|SetTaken false)))

(event OnComponentEndOverlap(BoxEndOfCover2_Right)
  (params (OverlappedComponent :type Primitive%20Component%20Object%20Reference) (OtherActor :type Actor%20Object%20Reference) (OtherComp :type Primitive%20Component%20Object%20Reference) (OtherBodyIndex :type Integer))
  (if (Utilities|DoesObjectImplementInterface OverlappedComponent (Variables|Default|GetCoverInterface))
    (Class|CoverInterface|EndOfCover(Message) OtherActor false false)
    (Variables|Default|SetTaken false)))

(event OnComponentBeginOverlap(BoxEndOfCover2_Left)
  (params (OverlappedComponent :type Primitive%20Component%20Object%20Reference) (OtherActor :type Actor%20Object%20Reference) (OtherComp :type Primitive%20Component%20Object%20Reference) (OtherBodyIndex :type Integer) (bFromSweep :type Boolean) (SweepResult :type Hit%20Result%20Structure%20%28by%20ref%29))
  (if (Utilities|DoesObjectImplementInterface OtherActor (Variables|Default|GetCoverInterface))
    (Class|CoverInterface|EndOfCover(Message) OtherActor true false)))

(event OnComponentBeginOverlap(BoxEndOfCover1_Left)
  (params (OverlappedComponent :type Primitive%20Component%20Object%20Reference) (OtherActor :type Actor%20Object%20Reference) (OtherComp :type Primitive%20Component%20Object%20Reference) (OtherBodyIndex :type Integer) (bFromSweep :type Boolean) (SweepResult :type Hit%20Result%20Structure%20%28by%20ref%29))
  (if (Utilities|DoesObjectImplementInterface OtherActor (Variables|Default|GetCoverInterface))
    (Class|CoverInterface|EndOfCover(Message) OtherActor true false)))

(event OnComponentEndOverlap(BoxEndOfCover1_Left)
  (params (OverlappedComponent :type Primitive%20Component%20Object%20Reference) (OtherActor :type Actor%20Object%20Reference) (OtherComp :type Primitive%20Component%20Object%20Reference) (OtherBodyIndex :type Integer))
  (if (Utilities|DoesObjectImplementInterface OverlappedComponent (Variables|Default|GetCoverInterface))
    (Class|CoverInterface|EndOfCover(Message) OtherActor false false)
    (Variables|Default|SetTaken false)))

(event OnComponentBeginOverlap(BoxEndOfCover1_Right)
  (params (OverlappedComponent :type Primitive%20Component%20Object%20Reference) (OtherActor :type Actor%20Object%20Reference) (OtherComp :type Primitive%20Component%20Object%20Reference) (OtherBodyIndex :type Integer) (bFromSweep :type Boolean) (SweepResult :type Hit%20Result%20Structure%20%28by%20ref%29))
  (if (Utilities|DoesObjectImplementInterface OtherActor (Variables|Default|GetCoverInterface))
    (Class|CoverInterface|EndOfCover(Message) OtherActor false true)))

(event Custom|IsTaken
  (Utilities|IsValid (Variables|Default|GetActorRef)
    (:Is%20Not%20Valid
      (Variables|Default|SetTaken false))))

(event EventBeginPlay
  (Utilities|Time|SetTimerbyEvent (delegate Custom|IsTaken) 2.0 true))

(fn ConstructionScript
  (Components|StaticMesh|SetStaticMesh (Variables|Default|GetStaticMesh) (Variables|Default|GetMesh)))
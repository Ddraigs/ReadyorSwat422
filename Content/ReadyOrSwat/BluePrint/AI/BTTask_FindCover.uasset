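; Behavior tree task that picks the nearest valid cover point for an AI pawn relative to the player.
; It sphere-overlaps Cover actors around the pawn and tests both arrows on each.
; An arrow qualifies if it faces the player within an angle limit, keeps a minimum distance from them and beats the closest distance so far.
; The winner sets the move-to location and cover-available Blackboard keys; the task always finishes successfully.
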(event EventReceiveExecuteAI
  (params (OwnerController :type AI%20Controller%20Object%20Reference) (ControlledPawn :type Pawn%20Object%20Reference))
  (Class|BTFunctionLibrary|SetBlackboardValueasBool (Variables|Default|GetIsCoverablivable) false)
  (bind _output_get (Variables|Default|SetDistanceToCover (Variables|Default|GetMaxDistanceToCover)))
  (bind _output_get_2 (Variables|Default|SetSelfLoc (Transformation|GetActorLocation ControlledPawn)))
  (bind _outactors (Collision|SphereOverlapActors _output_get_2 _output_get (Utilities|Array|MakeArray "ObjectTypeQuery1") "/Game/ReadyOrSwat/BluePrint/AI/Cover.Cover_C"))
  (for _array_element _outactors
    (bind _ascover (Utilities|Casting|CastToCover _array_element))
    (Variables|Default|SetArrow1 (Variables|/Game/ReadyOrSwat/BluePrint/AI/Cover.Cover_C|GetArrow _ascover))
    (Variables|Default|SetArrow2 (Variables|/Game/ReadyOrSwat/BluePrint/AI/Cover.Cover_C|GetArrow1 _ascover))
    (Utilities|FlowControl|Sequence
      (:then_0
        (if (CallFunction|CheckRotandDistance (Variables|Default|GetArrow1))
          (AI|BehaviorTree|SetBlackboardValueasVector (Variables|Default|GetMoveToLoc) (Transformation|GetWorldLocation (Variables|Default|GetArrow1)))
          (Class|BTFunctionLibrary|SetBlackboardValueasBool (Variables|Default|GetIsCoverablivable) true)))
      (:then_1
        (if (CallFunction|CheckRotandDistance (Variables|Default|GetArrow2))
          (AI|BehaviorTree|SetBlackboardValueasVector (Variables|Default|GetMoveToLoc) (Transformation|GetWorldLocation (Variables|Default|GetArrow2)))
          (Class|BTFunctionLibrary|SetBlackboardValueasBool (Variables|Default|GetIsCoverablivable) true)))))
  (AI|BehaviorTree|FinishExecute true))

(fn CheckRotandDistance
  (params (ArrowRefLocal :type Arrow%20Component%20Object%20Reference))
  (Variables|Default|SetArrowRefLocal ArrowRefLocal)
  (Variables|Default|SetPlayerCharLoc (Transformation|GetActorLocation (AI|BehaviorTree|GetBlackboardValueasActor (Variables|Default|GetPlayerChar))))
  (if (Math|Boolean|ANDBoolean (< (Class|KismetMathLibrary|DegAcos (Math|Vector|DotProduct (Math|Vector|GetForwardVector (Transformation|GetWorldRotation (Variables|Default|GetArrowRefLocal))) (Math|Rotator|GetRotationXVector (Math|Rotator|FindLookatRotation (Transformation|GetWorldLocation (Variables|Default|GetArrowRefLocal)) (Variables|Default|GetPlayerCharLoc))))) 75.0) (< (Math|Vector|VectorLength (- (Transformation|GetWorldLocation (Variables|Default|GetArrowRefLocal)) (Variables|Default|GetSelfLoc))) (Variables|Default|GetDistanceToCover)) (> (Math|Vector|VectorLength (- (Transformation|GetWorldLocation (Variables|Default|GetArrowRefLocal)) (Variables|Default|GetPlayerCharLoc))) (Variables|Default|GetMinDistanceAwayFromPlayer)))
    (Variables|Default|SetDistanceToCover (Math|Vector|VectorLength (- (Transformation|GetWorldLocation (Variables|Default|GetArrowRefLocal)) (Variables|Default|GetSelfLoc))))
    (return true)
    (else
      (return false))))
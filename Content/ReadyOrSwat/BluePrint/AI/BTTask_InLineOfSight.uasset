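; Behavior tree task that checks whether RoS_Player is directly in front of the AI pawn.
; It casts a short line trace along the pawn's forward vector against world and pawn objects, with debug drawing on.
; It sets the CanSeePlayer blackboard bool true only if the first hit is the player, false otherwise, then always finishes successfully.
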(event EventReceiveExecuteAI
  (params (OwnerController :type AI%20Controller%20Object%20Reference) (ControlledPawn :type Pawn%20Object%20Reference))
  (bind _returnvalue (Transformation|GetActorLocation ControlledPawn))
  (bind _canseeplayer (Variables|Default|GetCanSeePlayer))
  (bind (_outhit _returnvalue_2) (Collision|LineTraceForObjects _returnvalue (+ _returnvalue (* (Math|Vector|GetForwardVector (Transformation|GetActorRotation ControlledPawn)) 5e+02)) (Utilities|Array|MakeArray "ObjectTypeQuery1" "ObjectTypeQuery2" "ObjectTypeQuery3") false (Utilities|Array|MakeArray ControlledPawn) "ForDuration"))
  (if _returnvalue_2
    (Utilities|Casting|CastToRoS_Player (.HitActor (Collision|BreakHitResult _outhit))
      (:then
        (Class|BTFunctionLibrary|SetBlackboardValueasBool _canseeplayer true))
      (:CastFailed
        (Class|BTFunctionLibrary|SetBlackboardValueasBool _canseeplayer false :!label _label)))
    (else
      (goto _label)))
  (AI|BehaviorTree|FinishExecute true))
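; AI controller for the Terry enemy AI, which selects a behavior tree to match a skill level.
; The BHT_Skill event takes a Skill value and runs the basic, medium-skilled or high-skilled Terry tree by threshold.
; The perception update event is empty; the logic that clears the CanSeePlayer blackboard key when sight of the player is lost is disconnected and never runs.
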(event OnTargetPerceptionUpdated(AIPerception)
  (params (Actor :type Actor%20Object%20Reference) (Stimulus :type AI%20Stimulus%20Structure)))

(event Custom|BHT_Skill
  (params (Skill :type Integer))
  (if (< Skill 34)
    (AI|RunBehaviorTree "/Game/ReadyOrSwat/BluePrint/AI/BT_AI_Terry.BT_AI_Terry")
    (elif (< Skill 68)
      (AI|RunBehaviorTree "/Game/ReadyOrSwat/BluePrint/AI/BT_AI_Terry_MediumSkilled.BT_AI_Terry_MediumSkilled")
      (elif (> Skill 67)
        (AI|RunBehaviorTree "/Game/ReadyOrSwat/BluePrint/AI/BT_AI_Terry_HighSkilled.BT_AI_Terry_HighSkilled")
        (else
          (AI|RunBehaviorTree "/Game/ReadyOrSwat/BluePrint/AI/BT_AI_Terry_HighSkilled.BT_AI_Terry_HighSkilled"))))))

(fn ConstructionScript)
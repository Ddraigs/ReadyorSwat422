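; Behavior tree service that copies AI_Char_Terry state into the blackboard for the AI's decision making.
; Each AI tick casts the controlled pawn, then updates the player-visibility flag and player reference only when they differ from the stored keys.
; AI skill and AI type are written once through a DoOnce.
; Despite the CombatStance name, it contains no stance logic itself.
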(event EventReceiveTickAI
  (params (OwnerController :type AI%20Controller%20Object%20Reference) (ControlledPawn :type Pawn%20Object%20Reference) (DeltaSeconds :type Float%20%28single-precision%29))
  (bind _canseeplayer (Variables|Default|GetCanSeePlayer))
  (bind _asai_char_terry (Utilities|Casting|CastToAI_Char_Terry ControlledPawn))
  (Utilities|FlowControl|Sequence
    (:then_0
      (if (not (Math|Boolean|Equal(Boolean) (Class|BTFunctionLibrary|GetBlackboardValueasBool _canseeplayer) (Variables|/Game/ReadyOrSwat/BluePrint/AI/AI_Char_Terry.AI_Char_Terry_C|GetB_SeePlayer _asai_char_terry)))
        (Class|BTFunctionLibrary|SetBlackboardValueasBool _canseeplayer (Variables|/Game/ReadyOrSwat/BluePrint/AI/AI_Char_Terry.AI_Char_Terry_C|GetB_SeePlayer _asai_char_terry))))
    (:then_1
      (if (not (== (Variables|/Game/ReadyOrSwat/BluePrint/AI/AI_Char_Terry.AI_Char_Terry_C|GetPlayerRef _asai_char_terry) (AI|BehaviorTree|GetBlackboardValueasActor (Variables|Default|GetPlayerReferance))))
        (Class|BTFunctionLibrary|SetBlackboardValueasObject (Variables|Default|GetPlayerReferance) (Variables|/Game/ReadyOrSwat/BluePrint/AI/AI_Char_Terry.AI_Char_Terry_C|GetPlayerRef _asai_char_terry))))
    (:then_2
      (Utilities|FlowControl|DoOnce false
        (:Completed
          (Class|BTFunctionLibrary|SetBlackboardValueasInt (Variables|Default|GetAISkill) (Variables|/Game/ReadyOrSwat/BluePrint/AI/AI_Char_Terry.AI_Char_Terry_C|GetAiSkill _asai_char_terry))
          (Class|BTFunctionLibrary|SetBlackboardValueasEnum (Variables|Default|GetAIType) (Variables|/Game/ReadyOrSwat/BluePrint/AI/AI_Char_Terry.AI_Char_Terry_C|GetAIType _asai_char_terry)))))))
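; Enemy "Terry" AI character, optionally an HVT, that seeds its controller's blackboard with morale, health and combat settings.
; Detection and combat alerts spread recursively to nearby Terrys through sphere overlaps.
; Timer-driven rifle fire spawns bullets in a skill-based spread cone, flagging reload after a random round count.
; Hits lower morale and health; death ragdolls the body, rewards the killing player, updates MissionGen counts, then destroys the actor.
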(event OnSeePawn(PawnSensing)
  (params (Pawn :type Pawn%20Object%20Reference))
  (CallFunction|SeePlayer Pawn))

(event OnHearNoise(PawnSensing)
  (params (Instigator :type Pawn%20Object%20Reference) (Location :type Vector%20%28by%20ref%29 :default "0, 0, 0") (Volume :type Float%20%28single-precision%29)))

(event Custom|FireWeapon
  (if (not (Variables|Health|GetIsDead?))
    (CallFunction|FireAssulteRife)))

(event Custom|FireAssulteRife
  (if (not (Variables|Cover|GetIsFiring))
    (Variables|Cover|SetIsAiming true)
    (Variables|Cover|SetIsFiring true)
    (Utilities|FlowControl|Delay 1.0)
    (Variables|Default|SetRifleGunBurstCount (Math|Random|RandomIntegerinRange 7 20))
    (CallFunction|FireRifleBurst)
    (bind _returnvalue (Utilities|Time|SetTimerbyEvent (delegate Custom|Fire_RifleBurst) 0.4 true))
    (Variables|Default|SetTimerHandle _returnvalue)))

(event Custom|StopFiringWeapon
  (bind _timerhandle (Variables|Default|GetTimerHandle))
  (Variables|Cover|SetIsAiming false)
  (Variables|Cover|SetIsFiring false)
  (Variables|Default|SetFireCount 0)
  (if (Utilities|Time|IsValidTimerHandle _timerhandle)
    (Utilities|Time|ClearandInvalidateTimerbyHandle _timerhandle)))

(event Custom|Reload
  (Animation|Montage|PlayMontage (Variables|Character|GetMesh) "/Game/ReadyOrSwat/Animation/Reload_Crouching_Montage.Reload_Crouching_Montage"))

(event Custom|Fire_RifleBurst
  (bind _arrow1 (Variables|Default|GetArrow1))
  (bind _returnvalue (Transformation|GetWorldLocation _arrow1))
  (if (< (Variables|Default|GetFireCount) (Variables|Default|GetRifleGunBurstCount))
    (Game|SpawnActorfromClass "/Game/ReadyOrSwat/BluePrint/Bullet.Bullet_C" (CallFunction|BulletSpawnTransform) "Undefined" 0 "NewEnumerator1" 0)
    (Effects|SpawnEmitteratLocation "/Game/StarterContent/Particles/P_Explosion.P_Explosion" _returnvalue "0, 0, 0" "0.200000,0.200000,0.200000")
    (Audio|PlaySoundatLocation "/Game/ReadyOrSwat/BluePrint/Inventory/Weapons/Sounds/M4A1Shot_TomFix.M4A1Shot_TomFix" _returnvalue "0, 0, 0" 1.0 1.0 0.0 0 0 0)
    (Variables|Default|SetFireCount (+ (Variables|Default|GetFireCount) 1))
    (else
      (AI|Components|Blackboard|SetValueasBool (AI|GetBlackboard (AI|GetAIController self)) (Utilities|Name|MakeLiteralName "NeedToRealod") true)
      (Utilities|FlowControl|Delay 1.0)
      (Variables|Default|SetFireCount 0))))

(event EventBeginPlay
  (bind _self self)
  (bind _returnvalue (AI|GetAIController _self))
  (bind _returnvalue_2 (AI|GetBlackboard _returnvalue))
  (bind _asai_conroller_terry (Utilities|Casting|CastToAI_Conroller_Terry (AI|GetAIController self))
    (:then
      (Default|BHTSkill _asai_conroller_terry (Variables|Default|GetAiSkill))
      (AI|Components|Blackboard|SetValueasFloat _returnvalue_2 (Utilities|Name|MakeLiteralName "Moral") (Variables|Health|GetMoral))
      (AI|Components|Blackboard|SetValueasFloat _returnvalue_2 (Utilities|Name|MakeLiteralName "Health") (Variables|Health|GetHealth))
      (AI|Components|Blackboard|SetValueasFloat _returnvalue_2 (Utilities|Name|MakeLiteralName "WeaponRange") (Variables|Cover|GetWeaponRange))
      (AI|Components|Blackboard|SetValueasBool _returnvalue_2 (Utilities|Name|MakeLiteralName "DoorClosed") false)
      (AI|Components|Blackboard|SetValueasBool _returnvalue_2 (Utilities|Name|MakeLiteralName "IsHvt?") (Variables|Default|GetISHVT)))
    (:CastFailed
      (Development|PrintString "Welll im not controleld here"))))

(event EventDealDamage
  (params (Damage :type Float%20%28single-precision%29) (HitBoneName :type Name :default "None") (DamageInstergater :type Actor%20Object%20Reference))
  (CallFunction|FDeath Damage DamageInstergater)
  (if (Variables|Health|GetIsDead?)
    (bind _asro_s_player (Utilities|Casting|CastToRoS_Player DamageInstergater))
    (Utilities|FlowControl|Sequence
      (:then_0
        (Utilities|FlowControl|DoOnce false
          (:Completed
            (Variables|/Game/ReadyOrSwat/BluePrint/RoS_Player.RoS_Player_C|SetHoldoutExp _asro_s_player (+ (Variables|/Game/ReadyOrSwat/BluePrint/RoS_Player.RoS_Player_C|GetHoldoutExp _asro_s_player) (Variables|Default|GetEXPGive)))
            (Math|Integer|IncrementInt (Variables|/Game/ReadyOrSwat/BluePrint/RoS_Player.RoS_Player_C|GetPlayerKills _asro_s_player)
              (:%20%20
                (bind _outactors (Actor|GetAllActorsOfClass "/Game/ReadyOrSwat/BluePrint/Tasks/MissionGen.MissionGen_C"))
                (if (Variables|Default|GetISHVT)
                  (Math|Integer|DecrementInt (Variables|/Game/ReadyOrSwat/BluePrint/Tasks/MissionGen.MissionGen_C|GetHVTRemaining (Utilities|Array|Get(acopy) _outactors))
                    (:%20%20
                      _))
                  (else
                    (Math|Integer|DecrementInt (Variables|/Game/ReadyOrSwat/BluePrint/Tasks/MissionGen.MissionGen_C|GetTerryRemaining (Utilities|Array|Get(acopy) _outactors))
                      (:%20%20
                        _))))
                (CallFunction|StopFiringWeapon))))))
      (:then_1
        (CallFunction|StopFiringWeapon)
        (Utilities|FlowControl|Delay 1e+01)
        (Actor|DestroyActor)))))

(event EventIsCoverAvilable
  (params (IsCoverAvliable :type Boolean) (CoverRot :type Rotator :default "0, 0, 0"))
  (Variables|Cover|SetCoverAvilable IsCoverAvliable)
  (Variables|Default|SetCoverRot CoverRot))

(fn ConstructionScript)

(fn SettoCombat
  (params (Object :type Actor%20Object%20Reference))
  (if (not (Utilities|Enum|Equal(Enum) (Variables|Default|GetAIStatus) "NewEnumerator0"))
    (bind _asro_s_player (Utilities|Casting|CastToRoS_Player Object)
      (:then
        (Variables|Default|SetPlayerRef _asro_s_player)
        (Variables|Default|SetCombatready true)
        (bind _outactors (Collision|SphereOverlapActors (Transformation|GetActorLocation) (Variables|Default|GetCommsrange) (Utilities|Array|MakeArray "ObjectTypeQuery3") "AI_Char_Terry_C" (Utilities|Array|MakeArray self)))
        (for _array_element _outactors
          (bind _asai_char_terry (Utilities|Casting|CastToAI_Char_Terry _array_element))
          (CallFunction|SettoCombat _asai_char_terry (Variables|Default|GetPlayerRef))))
      (:CastFailed
        _)))
  (return))

(fn SetIsTakingCover
  (params (IsTakingCover :type Boolean))
  (if (not (Variables|Cover|GetIsAiming))
    (bind _output_get (Variables|Cover|SetIsTakingCover IsTakingCover))
    (if _output_get
      (Transformation|SetActorRotation (Variables|Default|GetCoverRot)))
    (else
      (Variables|Cover|SetIsTakingCover false))))

(fn SeePlayer
  (params (DetectedObject :type Actor%20Object%20Reference))
  (if (not (Variables|Default|GetB_SeePlayer))
    (bind _asro_s_player (Utilities|Casting|CastToRoS_Player DetectedObject)
      (:then
        (Variables|Default|SetPlayerRef _asro_s_player)
        (Variables|Default|SetB_SeePlayer true)
        (bind _outactors (Collision|SphereOverlapActors (Transformation|GetActorLocation) (Variables|Default|GetCommsrange) (Utilities|Array|MakeArray "ObjectTypeQuery3") "AI_Char_Terry_C" (Utilities|Array|MakeArray self)))
        (for _array_element _outactors
          (bind _asai_char_terry (Utilities|Casting|CastToAI_Char_Terry _array_element))
          (CallFunction|SeePlayer _asai_char_terry (Variables|Default|GetPlayerRef))))
      (:CastFailed
        _))
    (return)))

(fn HearPlayer
  (params (DetectedObject :type Actor%20Object%20Reference))
  (if (not (Variables|Default|GetB_HearPlayer))
    (bind _asro_s_player (Utilities|Casting|CastToRoS_Player DetectedObject)
      (:then
        (Variables|Default|SetPlayerRef _asro_s_player)
        (Variables|Default|SetB_HearPlayer true)
        (bind _outactors (Collision|SphereOverlapActors (Transformation|GetActorLocation) (Variables|Default|GetCommsrange) (Utilities|Array|MakeArray "ObjectTypeQuery3") "AI_Char_Terry_C" (Utilities|Array|MakeArray self)))
        (for _array_element _outactors
          (bind _asai_char_terry (Utilities|Casting|CastToAI_Char_Terry _array_element))
          (CallFunction|SeePlayer _asai_char_terry (Variables|Default|GetPlayerRef))))
      (:CastFailed
        _))
    (return)))

(fn MoralCalc
  (bind _output_get (Variables|Health|SetMoral (- (Variables|Health|GetMoral) 1e+02)))
  (AI|Components|Blackboard|SetValueasFloat (AI|GetBlackboard (AI|GetAIController self)) (Utilities|Name|MakeLiteralName "Moral") _output_get)
  (return))

(fn HealthCalc
  (params (DamgeIn :type Float%20%28single-precision%29))
  (bind _output_get (Variables|Health|SetHealth (- (Variables|Health|GetHealth) DamgeIn)))
  (AI|Components|Blackboard|SetValueasFloat (AI|GetBlackboard (AI|GetAIController self)) (Utilities|Name|MakeLiteralName "Health") _output_get)
  (return (<= _output_get 0.0)))

(fn AISkillAim
  (if (< (Variables|Default|GetAiSkill) 34)
    (return 45.0)
    (elif (< (Variables|Default|GetAiSkill) 67)
      (return 2e+01)
      (else
        (if (> (Variables|Default|GetAiSkill) 66)
          _
          (else
            _))
        (return 5.0)))))

(fn BulletSpawnTransform
  (bind _arrow1 (Variables|Default|GetArrow1))
  (bind _returnvalue (Transformation|GetWorldTransform _arrow1))
  (return (Math|Transform|MakeTransform (.location _returnvalue) (Math|Rotator|MakeRotfromX (Math|Random|RandomUnitVectorinConeinDegrees (Math|Vector|GetForwardVector (Pawn|GetControlRotation :!class /Script/Engine.Pawn)) (CallFunction|AISkillAim))) (.scale _returnvalue))))

(fn FDeath
  (params (DamgeIn :type Float%20%28single-precision%29) (DamageInstagator :type Object%20Object%20Reference))
  (CallFunction|MoralCalc)
  (bind _returnvalue (CallFunction|HealthCalc DamgeIn))
  (if _returnvalue
    (Variables|Health|SetIsDead? true)
    (Physics|SetSimulatePhysics (Variables|Character|GetMesh) true)
    (Collision|SetCollisionEnabled (Variables|Character|GetMesh) "QueryAndPhysics")
    (Collision|SetCollisionEnabled (Variables|Collision|GetCapsuleComponent) "NoCollision")
    (CallFunction|StopFiringWeapon)
    (return true)
    (else
      (return false))))

(fn DoorStopDoor)

(fn GetSquadPointLoc
  (Variables|Default|SetSqaudPointArray (Utilities|Array|MakeArray (Transformation|GetWorldLocation (Variables|Default|GetSqaudLoc_1)) (Transformation|GetWorldLocation (Variables|Default|GetSqaudLoc_2)) (Transformation|GetWorldLocation (Variables|Default|GetSqaudLoc_3)) (Transformation|GetWorldLocation (Variables|Default|GetSqaudLoc_4)) (Transformation|GetWorldLocation (Variables|Default|GetSqaudLoc_5)) (Transformation|GetWorldLocation (Variables|Default|GetSqaudLoc_6)) (Transformation|GetWorldLocation (Variables|Default|GetSqaudLoc_7)) (Transformation|GetWorldLocation (Variables|Default|GetSqaudLoc_8))))
  (return))
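; Behavior tree task that picks a random player as the target for the Terry AI character.
; If the blackboard already holds a valid player, it randomly keeps that player or re-rolls; otherwise it always rolls.
; The roll indexes all RoS_Player actors using the game mode's max player count rather than the array length, then stores the result on the pawn and blackboard.
; A failed cast leaves the task unfinished.
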(event EventReceiveExecuteAI
  (params (OwnerController :type AI%20Controller%20Object%20Reference) (ControlledPawn :type Pawn%20Object%20Reference))
  (Utilities|IsValid (AI|BehaviorTree|GetBlackboardValueasActor (Variables|Default|GetPlayerReferance))
    (:Is%20Valid
      (if (Math|Random|RandomBool)
        _
        (else
          (bind _asready_or_swat_game_mode (Utilities|Casting|CastToReadyOrSwatGameMode (Game|GetGameMode) :!label _label))
          (bind _outactors (Actor|GetAllActorsOfClass "/Game/ReadyOrSwat/BluePrint/RoS_Player.RoS_Player_C"))
          (bind _asai_char_terry (Utilities|Casting|CastToAI_Char_Terry ControlledPawn))
          (bind _output_get (Variables|/Game/ReadyOrSwat/BluePrint/AI/AI_Char_Terry.AI_Char_Terry_C|SetPlayerRef _asai_char_terry (Utilities|Array|Get(acopy) _outactors (Math|Random|RandomIntegerinRange 0 (- (Variables|/Game/ReadyOrSwat/BluePrint/ReadyOrSwatGameMode.ReadyOrSwatGameMode_C|GetMaxPlayercount _asready_or_swat_game_mode) 1)))))
          (Class|BTFunctionLibrary|SetBlackboardValueasObject (Variables|Default|GetPlayerReferance) _output_get))))
    (:Is%20Not%20Valid
      (goto _label)))
  (AI|BehaviorTree|FinishExecute true))
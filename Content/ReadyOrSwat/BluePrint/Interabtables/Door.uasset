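; Interactable door that players swing open or shut through a timeline driving mesh yaw, unless it is locked.
; Door stop events lock and unlock it; crowbarring clears the lock and blocks any further door stop.
; When AI_Terrance enters the trigger box, a door-stopped door gets a timed C4 spawned at its Destructible.
; Otherwise it snaps open, and it snaps shut four seconds after the AI leaves.
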(event OnComponentBeginOverlap(Box)
  (params (OverlappedComponent :type Primitive%20Component%20Object%20Reference) (OtherActor :type Actor%20Object%20Reference) (OtherComp :type Primitive%20Component%20Object%20Reference) (OtherBodyIndex :type Integer) (bFromSweep :type Boolean) (SweepResult :type Hit%20Result%20Structure%20%28by%20ref%29))
  (Utilities|Casting|CastToAI_Terrance OtherActor)
  (if (Variables|Default|GetHasDoorStop)
    (bind _returnvalue (Game|SpawnActorfromClass "/Game/ReadyOrSwat/BluePrint/Interabtables/C4Interactable.C4Interactable_C" (Transformation|GetWorldTransform (Variables|Default|GetDestructible)) "Undefined" 0 "50.000000,50.000000,50.000000" 0))
    (Default|StartTimer _returnvalue)
    (else
      (Transformation|SetRelativeRotation (Variables|Default|GetInteracableMesh) (Math|Rotator|MakeRotator 0.0 0.0 -3e+01) false false)
      (Variables|Default|SetDoorOpen true))))

(event OnComponentEndOverlap(Box)
  (params (OverlappedComponent :type Primitive%20Component%20Object%20Reference) (OtherActor :type Actor%20Object%20Reference) (OtherComp :type Primitive%20Component%20Object%20Reference) (OtherBodyIndex :type Integer))
  (Utilities|Casting|CastToAI_Terrance OtherActor)
  (Utilities|FlowControl|Delay 4.0)
  (Transformation|SetRelativeRotation (Variables|Default|GetInteracableMesh) (Math|Rotator|MakeRotator 0.0 0.0 9e+01) false false)
  (Variables|Default|SetDoorOpen false))

(event Custom|LockDoorStop
  (if (not (Variables|Default|GetCrowbared?))
    (Variables|Default|SetLocked? true)
    (Variables|Default|SetHasDoorStop true)))

(event Custom|UnlockDoorStop
  (Variables|Default|SetLocked? false)
  (Variables|Default|SetHasDoorStop false))

(event Custom|Crowbared
  (Variables|Default|SetCrowbared? true)
  (Variables|Default|SetLocked? false)
  (Variables|Default|SetHasDoorStop false))

(event EventUsed
  (params (InteractedActor :type Ro%20S%20Player%20Object%20Reference))
  (if (not (Variables|Default|GetLocked?))
    (if (Variables|Default|GetDoorOpen)
      (Variables|Default|SetDoorOpen false)
      (bind _doorrotamt (Timeline|Door Reverse)
        (:Update
          (Transformation|SetRelativeRotation (Variables|Default|GetInteracableMesh) (Math|Rotator|MakeRotator 0.0 0.0 _doorrotamt) false false)))
      (else
        (Variables|Default|SetDoorOpen true)
        (Timeline|Door Play)))))

(event EventTick
  (params (DeltaSeconds :type Float%20%28single-precision%29)))

(fn ConstructionScript
  (|CallParentFunction))
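; InteractableActor is an actor that player characters can interact with, exposing an empty Used event as the interaction hook.
; Its box trigger flags an overlapping RoSChar and hands it a self reference; leaving clears the flag but keeps the reference.
; The construction script applies the configurable box size, physics simulation and mass override to the box and mesh.
; Tick only stores the frame delta.
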(event OnComponentBeginOverlap(Box)
  (params (OverlappedComponent :type Primitive%20Component%20Object%20Reference) (OtherActor :type Actor%20Object%20Reference) (OtherComp :type Primitive%20Component%20Object%20Reference) (OtherBodyIndex :type Integer) (bFromSweep :type Boolean) (SweepResult :type Hit%20Result%20Structure%20%28by%20ref%29))
  (bind _asro_schar (Utilities|Casting|CastToRoSChar OtherActor))
  (if (== _asro_schar OtherActor)
    (Variables|/Game/ReadyOrSwat/BluePrint/RoSChar.RoSChar_C|SetInteractableOverLaped _asro_schar true)
    (Variables|/Game/ReadyOrSwat/BluePrint/RoSChar.RoSChar_C|SetInteractableRef _asro_schar self)))

(event OnComponentEndOverlap(Box)
  (params (OverlappedComponent :type Primitive%20Component%20Object%20Reference) (OtherActor :type Actor%20Object%20Reference) (OtherComp :type Primitive%20Component%20Object%20Reference) (OtherBodyIndex :type Integer))
  (bind _asro_schar (Utilities|Casting|CastToRoSChar OtherActor))
  (if (== _asro_schar OtherActor)
    (Variables|/Game/ReadyOrSwat/BluePrint/RoSChar.RoSChar_C|SetInteractableOverLaped _asro_schar false)))

(event Custom|Used
  (params (InteractedActor :type Ro%20S%20Player%20Object%20Reference)))

(event EventBeginPlay)

(event Collision|EventActorBeginOverlap
  (params (OtherActor :type Actor%20Object%20Reference)))

(event EventTick
  (params (DeltaSeconds :type Float%20%28single-precision%29))
  (Variables|Default|SetDelta DeltaSeconds))

(fn ConstructionScript
  (Components|Box|SetBoxExtent (Variables|Default|GetBox) (Variables|Default|GetBoxSizeVar) true)
  (Physics|SetSimulatePhysics (Variables|Default|GetInteracableMesh) (Variables|Default|GetIsSimulatingPhysics))
  (Class|PrimitiveComponent|SetMassOverrideinKg (Variables|Default|GetInteracableMesh) "None" (Variables|Default|GetMassOfObject) true))
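; Laser trip mine interactable that fires a cone of projectiles and destroys itself when triggered.
; On BeginPlay it traces forward from its arrow, draws a beam to the hit point and stretches the trigger box along it.
; Overlap by an AI_Char_Terry or RoS_Player spawns a burst of Bullet actors within a forward cone, but only the AI path spawns the explosion effect.
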(event OnComponentBeginOverlap(Box1)
  (params (OverlappedComponent :type Primitive%20Component%20Object%20Reference) (OtherActor :type Actor%20Object%20Reference) (OtherComp :type Primitive%20Component%20Object%20Reference) (OtherBodyIndex :type Integer) (bFromSweep :type Boolean) (SweepResult :type Hit%20Result%20Structure%20%28by%20ref%29))
  (Utilities|Casting|CastToAI_Char_Terry OtherActor
    (:then
      (Effects|SpawnEmitteratLocation "/Game/StarterContent/Particles/P_Explosion.P_Explosion" (Transformation|GetWorldLocation (Variables|Default|GetInteracableMesh)) "0, 0, 0" "2.000000,2.000000,2.000000"))
    (:CastFailed
      (Utilities|Casting|CastToRoS_Player OtherActor)))
  (for _index (range 0 70)
    (Game|SpawnActorfromClass "/Game/ReadyOrSwat/BluePrint/Bullet.Bullet_C" (CallFunction|SpawnTransform) "Undefined" 0 "NewEnumerator4" 0))
  (Components|DestroyComponent (Variables|Default|GetLasterBeamTrip))
  (Actor|DestroyActor))

(event EventBeginPlay
  (bind _arrow (Variables|Default|GetArrow))
  (bind _returnvalue (Transformation|GetWorldLocation _arrow))
  (|CallParentFunction)
  (Collision|SetCollisionEnabled (Variables|Default|GetBox1) "NoCollision")
  (bind _output_get (Variables|Default|SetBeamEndPoint (+ _returnvalue (* (Math|Vector|GetForwardVector _arrow) 5e+03))))
  (bind (_outhit _returnvalue_2) (Collision|LineTraceByChannel _returnvalue _output_get "TraceTypeQuery1" false 0 "None"))
  (if _returnvalue_2
    (Variables|Default|SetBeamEndPoint (.Location (Collision|BreakHitResult _outhit))))
  (CallFunction|CreateBeam (Transformation|GetWorldLocation (Variables|Default|GetArrow)) (Variables|Default|GetBeamEndPoint))
  (CallFunction|ScaleTriggerBox (Variables|Default|GetBeamEndPoint))
  (Collision|SetCollisionEnabled (Variables|Default|GetBox1) "QueryOnly"))

(event Collision|EventActorBeginOverlap
  (params (OtherActor :type Actor%20Object%20Reference))
  (|CallParentFunction OtherActor) ; This node is disabled and will not be called.\nDrag off pins to build functionality.
)

(event EventTick
  (params (DeltaSeconds :type Float%20%28single-precision%29))
  (|CallParentFunction DeltaSeconds) ; This node is disabled and will not be called.\nDrag off pins to build functionality.
)

(event EventUsed
  (params (InteractedActor :type Ro%20S%20Player%20Object%20Reference)))

(fn ConstructionScript
  (|CallParentFunction))

(fn SpawnTransform
  (return (Math|Transform|MakeTransform (.location (Transformation|GetWorldTransform (Variables|Default|GetArrow))) (Math|Rotator|MakeRotfromX (Math|Random|RandomUnitVectorinConeinDegrees (Math|Vector|GetForwardVector (Variables|Default|GetArrow)) 2e+01)))))

(fn CreateBeam
  (params (StartLoc :type Vector) (EndLoc :type Vector))
  (bind _returnvalue (Effects|SpawnEmitteratLocation "/Game/ReadyOrSwat/BluePrint/Interabtables/laster.laster" StartLoc))
  (bind _output_get (Variables|Default|SetLasterBeamTrip _returnvalue))
  (Class|ParticleSystemComponent|SetBeamEndPoint _output_get 0 EndLoc))

(fn ScaleTriggerBox
  (params (EndLoc :type Vector))
  (bind _box1 (Variables|Default|GetBox1))
  (bind _arrow (Variables|Default|GetArrow))
  (bind _returnvalue (Transformation|GetWorldLocation _arrow))
  (bind _returnvalue_2 (- EndLoc _returnvalue))
  (bind _returnvalue_3 (Math|Vector|VectorLength _returnvalue_2))
  (bind _returnvalue_4 (/ _returnvalue_3 2.0))
  (bind _returnvalue_5 (Math|Vector|MakeVector _returnvalue_4 1.0 1.0))
  (Transformation|SetRelativeScale3D _box1 _returnvalue_5)
  (Transformation|SetRelativeLocation _box1 (+ (Variables|/Script/Engine.SceneComponent|GetRelativeLocation _box1) _returnvalue_5) false false))
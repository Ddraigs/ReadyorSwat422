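; C4 interactable that acts as a timed explosive for blowing up destructible objects.
; StartTimer, not called within this graph (Used is empty), schedules BOOM after C4Timer, which spawns an explosion at the mesh.
; A sphere trace finds Destructible objects and applies radial damage once per hit.
; The actor destroys itself only when the trace hits; otherwise it prints a debug message and remains.
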(event Custom|StartTimer
  (Utilities|Time|SetTimerbyEvent (delegate Custom|BOOM!) (Variables|Default|GetC4Timer)))

(event Custom|BOOM!
  (bind _interacablemesh (Variables|Default|GetInteracableMesh))
  (bind _returnvalue (Transformation|GetWorldLocation _interacablemesh))
  (Effects|SpawnEmitteratLocation "/Game/StarterContent/Particles/P_Explosion.P_Explosion" (Transformation|GetWorldLocation (Variables|Default|GetInteracableMesh)) "0, 0, 0" "5.000000,5.000000,5.000000")
  (bind (_outhits _returnvalue_2) (Collision|MultiSphereTraceForObjects _returnvalue "0, 0, 0" 2.5e+02 (Utilities|Array|MakeArray "ObjectTypeQuery6") false 0 "None"))
  (if _returnvalue_2
    (for _array_element _outhits
      (Class|GameplayStatics|ApplyRadialDamagewithFalloff (.HitActor (Collision|BreakHitResult _array_element)) 5e+02 5e+02 _returnvalue 2.5e+02 5e+02 0.25 0 0 self (Game|GetInstigatorController) "ECC_Vehicle"))
    (Actor|DestroyActor)
    (else
      (Development|PrintString "I Aint hit shit"))))

(event EventBeginPlay
  (|CallParentFunction) ; This node is disabled and will not be called.\nDrag off pins to build functionality.
)

(event Collision|EventActorBeginOverlap
  (params (OtherActor :type Actor%20Object%20Reference))
  (|CallParentFunction OtherActor) ; This node is disabled and will not be called.\nDrag off pins to build functionality.
)

(event EventTick
  (params (DeltaSeconds :type Float%20%28single-precision%29))
  (|CallParentFunction DeltaSeconds) ; This node is disabled and will not be called.\nDrag off pins to build functionality.
)

(event EventUsed
  (params (InteractedActor :type Ro%20S%20Player%20Object%20Reference)))

(fn ConstructionScript
  (|CallParentFunction))
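; SledgeHammer is an interactable tool Blueprint that breaks destructible objects on impact.
; When its Box component registers a hit, it casts the hit component to a DestructibleComponent.
; On a match, it applies radial damage with falloff at the impact point and adds a constant-falloff radial force to that component.
; Debug prints trace the hit and successful cast, and the construction script only calls its parent.
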(event OnComponentHit(Box)
  (params (HitComponent :type Primitive%20Component%20Object%20Reference) (OtherActor :type Actor%20Object%20Reference) (OtherComp :type Primitive%20Component%20Object%20Reference) (NormalImpulse :type Vector :default "0, 0, 0") (Hit :type Hit%20Result%20Structure%20%28by%20ref%29))
  (bind (_bblockinghit _binitialoverlap _time _distance _location _impactpoint _normal _impactnormal _physmat _hitactor _hitcomponent) (Collision|BreakHitResult Hit))
  (Development|PrintString "Event HIt")
  (bind _asdestructible_component (Utilities|Casting|CastToDestructibleComponent _hitcomponent))
  (Development|PrintString "Hello")
  (if (== _asdestructible_component _hitcomponent)
    (Class|GameplayStatics|ApplyRadialDamagewithFalloff 2e+02 1e+02 _location 1e+02 2e+02 0.25 0 0 0 0 "ECC_Visibility")
    (Physics|AddRadialForce _hitcomponent _location 0.0 0.0 "RIF_Constant" false)))

(event EventBeginPlay
  (|CallParentFunction) ; This node is disabled and will not be called.\nDrag off pins to build functionality.
)

(event Collision|EventActorBeginOverlap
  (params (OtherActor :type Actor%20Object%20Reference))
  (|CallParentFunction OtherActor) ; This node is disabled and will not be called.\nDrag off pins to build functionality.
)

(event EventTick
  (params (DeltaSeconds :type Float%20%28single-precision%29))
  (|CallParentFunction DeltaSeconds) ; This node is disabled and will not be called.\nDrag off pins to build functionality.
)

(fn ConstructionScript
  (|CallParentFunction))
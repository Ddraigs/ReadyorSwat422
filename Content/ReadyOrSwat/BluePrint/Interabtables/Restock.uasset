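; Interactable restock station that shows a restock menu on its widget component to one player at a time.
; Using it locks that player's movement, enables UI mode and creates a RestockWidget owned by the station.
; Closing, also triggered by leaving the box, releases the player and refreshes the weapon mesh.
; IncreaseAmmos tops up weapon and gear counts; the input-mode restore calls, including UIFIX, are unwired.
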(event OnComponentEndOverlap(Box)
  (params (OverlappedComponent :type Primitive%20Component%20Object%20Reference) (OtherActor :type Actor%20Object%20Reference) (OtherComp :type Primitive%20Component%20Object%20Reference) (OtherBodyIndex :type Integer))
  (if (== (Variables|Default|GetPlayerRef) OtherActor)
    (CallFunction|CloseMenu)))

(event Custom|Close%20menu
  (bind _playerref (Variables|Default|GetPlayerRef))
  (bind _widget (Variables|Default|GetWidget))
  (Rendering|SetVisibility _widget false false)
  (Variables|/Game/ReadyOrSwat/BluePrint/RoSChar.RoSChar_C|SetMovementDisabled? _playerref false)
  (Variables|/Game/ReadyOrSwat/BluePrint/RoS_Player.RoS_Player_C|SetUIMode _playerref false)
  (Default|SetActivePlayerWeaponMesh (Variables|Default|GetPlayerRef))
  (Variables|Default|SetB_InUse? false)
  (Widget|RemovefromParent (UserInterface|GetUserWidgetObject _widget)))

(event EventBeginPlay
  (|CallParentFunction))

(event EventUsed
  (params (InteractedActor :type Ro%20S%20Player%20Object%20Reference))
  (if (not (Variables|Default|GetB_InUse?))
    (Variables|Default|SetB_InUse? true)
    (bind _output_get (Variables|Default|SetPlayerRef InteractedActor))
    (if (Utilities|IsValid _output_get)
      (Variables|/Game/ReadyOrSwat/BluePrint/RoSChar.RoSChar_C|SetMovementDisabled? (Variables|Default|GetPlayerRef) true)
      (Variables|/Game/ReadyOrSwat/BluePrint/RoS_Player.RoS_Player_C|SetUIMode (Variables|Default|GetPlayerRef) true)
      (bind _returnvalue (UserInterface|CreateWidget "/Game/ReadyOrSwat/BluePrint/Interabtables/RestockWidget.RestockWidget_C" (Game|GetPlayerController (Variables|/Game/ReadyOrSwat/BluePrint/RoS_Player.RoS_Player_C|GetPlayerControllerIndex (Variables|Default|GetPlayerRef))) (Variables|/Game/ReadyOrSwat/BluePrint/RoS_Player.RoS_Player_C|GetPlayerControllerIndex (Variables|Default|GetPlayerRef)) self))
      (UserInterface|SetWidget (Variables|Default|GetWidget) _returnvalue)
      (Rendering|SetVisibility (Variables|Default|GetWidget) true false)
      (Input|SetInputModeGameandUI (Game|GetPlayerController (Variables|/Game/ReadyOrSwat/BluePrint/RoS_Player.RoS_Player_C|GetPlayerControllerIndex (Variables|Default|GetPlayerRef))) _returnvalue "DoNotLock" true)
      (else
        (Development|PrintString "Player ref invaild you")))))

(fn ConstructionScript
  (|CallParentFunction))

(fn IncreaseAmmos
  (bind _playerref (Variables|Default|GetPlayerRef))
  (Variables|/Game/ReadyOrSwat/BluePrint/RoSChar.RoSChar_C|SetPrimaryAmmo _playerref (+ (Variables|/Game/ReadyOrSwat/BluePrint/RoSChar.RoSChar_C|GetPrimaryAmmo _playerref) (Variables|Restocks|GetAmmoToGive)))
  (Variables|/Game/ReadyOrSwat/BluePrint/RoSChar.RoSChar_C|SetSecondaryAmmo _playerref (+ (Variables|/Game/ReadyOrSwat/BluePrint/RoSChar.RoSChar_C|GetSecondaryAmmo _playerref) (Variables|Restocks|GetAmmoToGive)))
  (Variables|/Game/ReadyOrSwat/BluePrint/RoSChar.RoSChar_C|SetGearSlot1Ammount _playerref (+ (Variables|/Game/ReadyOrSwat/BluePrint/RoSChar.RoSChar_C|GetGearSlot1Ammount _playerref) (Variables|Restocks|GetGearAmmoToGive)))
  (Variables|/Game/ReadyOrSwat/BluePrint/RoSChar.RoSChar_C|SetGearSlot2Ammount _playerref (+ (Variables|/Game/ReadyOrSwat/BluePrint/RoSChar.RoSChar_C|GetGearSlot2Max _playerref) (Variables|Restocks|GetGearAmmoToGive))))

(fn UIFIX
  (params (PlayerIndex :type Integer))
  (bind _returnvalue (Game|GetPlayerController PlayerIndex))
  (Utilities|IsValid _returnvalue
    (:Is%20Valid
      (bind _asro_s_player (Utilities|Casting|CastToRoS_Player (Pawn|GetControlledPawn _returnvalue)))
      (if (Variables|/Game/ReadyOrSwat/BluePrint/RoS_Player.RoS_Player_C|GetUIMode _asro_s_player)
        _
        (else
          (Input|SetInputModeGameOnly _returnvalue))))
    (:Is%20Not%20Valid
      _))
  (return))
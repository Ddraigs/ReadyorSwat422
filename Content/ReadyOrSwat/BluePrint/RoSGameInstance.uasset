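; Game instance for ReadyOrSwat that holds the player's character customisation in a PlayerLooks struct.
; SetLooks and GetLooks switch on a selection to write or read one field: gender, head, back, eye and mouth shape values, or colour.
; GetLooks returns hardcoded IsFemale flags instead of reading the stored gender.
; SetLooks always writes zero for Eye Sinus, ignoring the passed value.
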(fn GetLooks
  (params (Selection :type E_Playerlooks%20Enum :default "NewEnumerator0"))
  (bind _playerlooks (Variables|Default|GetPlayerLooks))
  (bind (_female_ _colour _maleheadshape1 _maleheadshape2 _maleheadshape3 _backshape _eyesize _eyetype1 _eyetype2 _eyesinus _mouthsize _lipvolume) (Utilities|Struct|BreakPlayerLooks _playerlooks))
  (switch Utilities|FlowControl|Switch|SwitchonE_Playerlooks Selection
    (:NewEnumerator0
      (return true 0.0 ""))
    (:NewEnumerator1
      (return false _maleheadshape1 ""))
    (:NewEnumerator2
      (return false _maleheadshape2 ""))
    (:NewEnumerator3
      (return false _maleheadshape3 ""))
    (:NewEnumerator5
      (return true _backshape ""))
    (:NewEnumerator6
      (return false _eyesize ""))
    (:NewEnumerator7
      (return false _eyetype1 ""))
    (:NewEnumerator8
      (return false _eyetype2 ""))
    (:NewEnumerator9
      (return true _eyesinus ""))
    (:NewEnumerator10
      (return false _mouthsize ""))
    (:NewEnumerator11
      (return false _lipvolume ""))
    (:NewEnumerator13
      (return false 0.0 _colour))))

(fn SetLooks
  (params (Selection :type E_Playerlooks%20Enum :default "NewEnumerator0") (Valuein :type Float%20%28single-precision%29) (BoolIn :type Boolean) (Colour :type Color%20Structure))
  (bind _playerlooks (Variables|Default|GetPlayerLooks))
  (switch Utilities|FlowControl|Switch|SwitchonE_Playerlooks Selection
    (:NewEnumerator0
      (Utilities|Struct|SetmembersinPlayerLooks _playerlooks BoolIn))
    (:NewEnumerator1
      (Utilities|Struct|SetmembersinPlayerLooks _playerlooks Valuein))
    (:NewEnumerator2
      (Utilities|Struct|SetmembersinPlayerLooks _playerlooks Valuein))
    (:NewEnumerator3
      (Utilities|Struct|SetmembersinPlayerLooks _playerlooks Valuein))
    (:NewEnumerator5
      (Utilities|Struct|SetmembersinPlayerLooks _playerlooks Valuein))
    (:NewEnumerator6
      (Utilities|Struct|SetmembersinPlayerLooks _playerlooks Valuein))
    (:NewEnumerator7
      (Utilities|Struct|SetmembersinPlayerLooks _playerlooks Valuein))
    (:NewEnumerator8
      (Utilities|Struct|SetmembersinPlayerLooks _playerlooks Valuein))
    (:NewEnumerator9
      (Utilities|Struct|SetmembersinPlayerLooks _playerlooks 0.0))
    (:NewEnumerator10
      (Utilities|Struct|SetmembersinPlayerLooks _playerlooks Valuein))
    (:NewEnumerator11
      (Utilities|Struct|SetmembersinPlayerLooks _playerlooks Valuein))
    (:NewEnumerator13
      (Utilities|Struct|SetmembersinPlayerLooks _playerlooks Colour)))
  (return))
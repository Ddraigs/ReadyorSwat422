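; Whiteboard Blueprint that lets markings be drawn onto a render target at a given 2D location.
; BeginPlay creates a dynamic instance of the marker material and clears the render target to opaque black.
; DrawOnWhiteBoard checks that PlayerIndex matches PlayersWhiteBoard, passes the location to the material's DrawLoc parameter, then draws that material into the render target.
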(event Custom|DrawOnWhiteBoard
  (params (LocToDraw :type Vector%202D%20Structure))
  (bind _whiteboardmarker_mi (Variables|Default|GetWhiteBoardMarker_Mi))
  (if (== (Variables|Default|GetPlayerIndex) (Variables|Default|GetPlayersWhiteBoard))
    (Rendering|Material|SetVectorParameterValue _whiteboardmarker_mi "DrawLoc" (Math|Conversions|ToLinearColor(Vector) (Math|Conversions|ToVector(Vector2D) LocToDraw)) :!class /Script/Engine.MaterialInstanceDynamic)
    (Rendering|DrawMaterialtoRenderTarget (Variables|Default|GetTextureRenderTarget) _whiteboardmarker_mi)))

(event EventBeginPlay
  (bind _returnvalue (Rendering|Material|CreateDynamicMaterialInstance "/Game/ReadyOrSwat/BluePrint/WhiteBoard/WhiteBoardMarker.WhiteBoardMarker" "None" :!class /Script/Engine.KismetMaterialLibrary))
  (Variables|Default|SetWhiteBoardMarker_Mi _returnvalue)
  (Rendering|ClearRenderTarget2D (Variables|Default|GetTextureRenderTarget)))

(event Collision|EventActorBeginOverlap
  (params (OtherActor :type Actor%20Object%20Reference)))

(event EventTick
  (params (DeltaSeconds :type Float%20%28single-precision%29)))

(fn ConstructionScript)
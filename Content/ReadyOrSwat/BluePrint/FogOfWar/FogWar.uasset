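; Fog-of-war actor that shows a scaled static mesh and manages the render target holding the fog state.
; On BeginPlay it creates a dynamic instance of the SubFog material, clears the render target to opaque black and makes the mesh visible.
; DrawSubtract passes a 2D location into the material's DrawLoc parameter, then draws that material to the render target to update the fog there.
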(event Custom|DrawSubtract
  (params (Value :type Vector%202D%20Structure))
  (Rendering|Material|SetVectorParameterValue (Variables|Default|GetSubtract_mi) "DrawLoc" (Math|Conversions|ToLinearColor(Vector) (Math|Conversions|ToVector(Vector2D) Value)) :!class /Script/Engine.MaterialInstanceDynamic)
  (Rendering|DrawMaterialtoRenderTarget "/Game/ReadyOrSwat/BluePrint/FogOfWar/FowRender.FowRender" (Variables|Default|GetSubtract_mi)))

(event EventBeginPlay
  (bind _returnvalue (Rendering|Material|CreateDynamicMaterialInstance "/Game/ReadyOrSwat/BluePrint/FogOfWar/SubFog.SubFog" "None" :!class /Script/Engine.KismetMaterialLibrary))
  (Variables|Default|SetSubtract_mi _returnvalue)
  (Rendering|ClearRenderTarget2D "/Game/ReadyOrSwat/BluePrint/FogOfWar/FowRender.FowRender")
  (Rendering|SetVisibility (Variables|Default|GetStaticMesh) true false))

(event Collision|EventActorBeginOverlap
  (params (OtherActor :type Actor%20Object%20Reference)))

(event EventTick
  (params (DeltaSeconds :type Float%20%28single-precision%29)))

(fn ConstructionScript
  (Transformation|SetWorldScale3D (Variables|Default|GetStaticMesh) (Variables|Default|GetScale)))
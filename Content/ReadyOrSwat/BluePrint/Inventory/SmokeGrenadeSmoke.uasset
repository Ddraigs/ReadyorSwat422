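; Smoke cloud actor for the smoke grenade that impairs the sight of AI_Char_Terry characters.
; On BeginPlay it activates two particle systems, then a 15-second timer deactivates them and destroys the actor.
; A box volume sets an overlapping Terry's PawnSensing sight radius to a very short range.
; End overlap writes the same short radius, so the original sight range is not restored here.
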(event OnComponentBeginOverlap(Box)
  (params (OverlappedComponent :type Primitive%20Component%20Object%20Reference) (OtherActor :type Actor%20Object%20Reference) (OtherComp :type Primitive%20Component%20Object%20Reference) (OtherBodyIndex :type Integer) (bFromSweep :type Boolean) (SweepResult :type Hit%20Result%20Structure%20%28by%20ref%29))
  (bind _asai_char_terry (Utilities|Casting|CastToAI_Char_Terry OtherActor))
  (Variables|/Script/AIModule.PawnSensingComponent|SetSightRadius (Variables|/Game/ReadyOrSwat/BluePrint/AI/AI_Char_Terry.AI_Char_Terry_C|GetPawnSensing _asai_char_terry) 1e+01))

(event OnComponentEndOverlap(Box)
  (params (OverlappedComponent :type Primitive%20Component%20Object%20Reference) (OtherActor :type Actor%20Object%20Reference) (OtherComp :type Primitive%20Component%20Object%20Reference) (OtherBodyIndex :type Integer))
  (bind _asai_char_terry (Utilities|Casting|CastToAI_Char_Terry OtherActor))
  (Variables|/Script/AIModule.PawnSensingComponent|SetSightRadius (Variables|/Game/ReadyOrSwat/BluePrint/AI/AI_Char_Terry.AI_Char_Terry_C|GetPawnSensing _asai_char_terry) 1e+01))

(event Custom|Stop
  (Components|Activation|Deactivate (Variables|Default|GetParticleSystem1))
  (Actor|DestroyActor))

(event EventBeginPlay
  (Components|Activation|Activate (Variables|Default|GetParticleSystem) true)
  (Utilities|Time|SetTimerbyEvent (delegate Custom|Stop) 15.0))

(event Collision|EventActorBeginOverlap
  (params (OtherActor :type Actor%20Object%20Reference)))

(event EventTick
  (params (DeltaSeconds :type Float%20%28single-precision%29)))

(fn ConstructionScript)
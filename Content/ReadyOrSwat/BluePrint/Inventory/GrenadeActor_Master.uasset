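; Base thrown grenade actor whose GrenadeType selects Frag, Smoke or Flash, setting its mesh and projectile speed at construction.
; A timer started on BeginPlay triggers Boom, which branches on that type.
; Frag radially damages overlapped destructibles and, per destructible hit, sprays randomly aimed Bullet actors as shrapnel with explosion effects.
; Smoke spawns a smoke actor; Flash disables nearby AI_Terrance sight and hearing perception, restoring sight first, then hearing.
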(event Custom|Boom
  (bind _returnvalue (Transformation|GetActorLocation))
  (bind _returnvalue_2 (Transformation|GetActorLocation))
  (bind _damage (Variables|Default|GetDamage))
  (Development|PrintString (Utilities|String|ToString(Float) (Variables|Default|GetDamage)))
  (Development|PrintString "arrived at boom")
  (switch Utilities|FlowControl|Switch|SwitchonE_Grenades (Variables|Default|GetGrenadeType)
    (:NewEnumerator0
      (bind _outactors (Collision|SphereOverlapActors (Transformation|GetActorLocation) 0.0 (Utilities|Array|MakeArray "ObjectTypeQuery1" "ObjectTypeQuery2" "ObjectTypeQuery6") 0))
      (for _array_element _outactors
        (bind _asdestructible_actor (Utilities|Casting|CastToDestructibleActor _array_element))
        (Class|GameplayStatics|ApplyRadialDamagewithFalloff _asdestructible_actor _damage _damage (Transformation|GetActorLocation) 2.5e+02 0.0 0.0 0 0 0 0 "ECC_Visibility")
        (for _index (range 0 (Math|Random|RandomIntegerinRange 20 66))
          (Game|SpawnActorfromClass "/Game/ReadyOrSwat/BluePrint/Bullet.Bullet_C" (Math|Transform|MakeTransform _returnvalue_2 (Math|Random|RandomRotator true) "1,1,1") "Undefined" 0 "NewEnumerator4" (Game|GetInstigator))
          (Effects|SpawnEmitteratLocation "/Game/StarterContent/Particles/P_Explosion.P_Explosion" _returnvalue_2))
        (Actor|DestroyActor))
      (Actor|DestroyActor))
    (:NewEnumerator1
      (Game|SpawnActorfromClass "/Game/ReadyOrSwat/BluePrint/Inventory/SmokeGrenadeSmoke.SmokeGrenadeSmoke_C" (Transformation|GetActorTransform) "Undefined" 0 0)
      (Actor|DestroyActor))
    (:NewEnumerator3
      (Effects|SpawnEmitteratLocation "/Game/StarterContent/Particles/P_Sparks.P_Sparks" _returnvalue)
      (bind _outactors_2 (Collision|SphereOverlapActors _returnvalue (Variables|Default|GetRadius) (Utilities|Array|MakeArray "ObjectTypeQuery3") 0))
      (bind _output_get (Variables|Default|SetEffectedTargets _outactors_2))
      (for _array_element_2 _output_get
        (bind _asai_terrance (Utilities|Casting|CastToAI_Terrance _array_element_2))
        (bind _asterrance_controller_ai (Utilities|Casting|CastToTerrance_Controller_Ai (Pawn|GetController _asai_terrance)))
        (Class|AIPerceptionComponent|SetSenseEnabled (Variables|/Game/ReadyOrSwat/BluePrint/AI_Terrance/Terrance_Controller_Ai.Terrance_Controller_Ai_C|GetAIPerception _asterrance_controller_ai) "/Script/AIModule.AISense_Sight" false)
        (Class|AIPerceptionComponent|SetSenseEnabled (Variables|/Game/ReadyOrSwat/BluePrint/AI_Terrance/Terrance_Controller_Ai.Terrance_Controller_Ai_C|GetAIPerception _asterrance_controller_ai) "/Script/AIModule.AISense_Hearing" false))
      (Utilities|FlowControl|Delay 5.0)
      (for _array_element_3 (Variables|Default|GetEffectedTargets)
        (bind _asai_terrance_2 (Utilities|Casting|CastToAI_Terrance _array_element_3))
        (bind _asterrance_controller_ai_2 (Utilities|Casting|CastToTerrance_Controller_Ai (Pawn|GetController _asai_terrance_2)))
        (Class|AIPerceptionComponent|SetSenseEnabled (Variables|/Game/ReadyOrSwat/BluePrint/AI_Terrance/Terrance_Controller_Ai.Terrance_Controller_Ai_C|GetAIPerception _asterrance_controller_ai_2) "/Script/AIModule.AISense_Sight" true))
      (Utilities|FlowControl|Delay 5.0)
      (for _array_element_4 (Variables|Default|GetEffectedTargets)
        (bind _asai_terrance_3 (Utilities|Casting|CastToAI_Terrance _array_element_4))
        (bind _asterrance_controller_ai_3 (Utilities|Casting|CastToTerrance_Controller_Ai (Pawn|GetController _asai_terrance_3)))
        (Class|AIPerceptionComponent|SetSenseEnabled (Variables|/Game/ReadyOrSwat/BluePrint/AI_Terrance/Terrance_Controller_Ai.Terrance_Controller_Ai_C|GetAIPerception _asterrance_controller_ai_3) "/Script/AIModule.AISense_Hearing" true))
      (Actor|DestroyActor))))

(event EventBeginPlay
  (Utilities|FlowControl|Delay 0.2)
  (Utilities|Time|SetTimerbyEvent (delegate Custom|Boom) 5.0))

(event Collision|EventActorBeginOverlap
  (params (OtherActor :type Actor%20Object%20Reference)))

(event EventTick
  (params (DeltaSeconds :type Float%20%28single-precision%29)))

(fn ConstructionScript
  (bind _staticmesh (Variables|Default|GetStaticMesh))
  (Variables|/Script/Engine.ProjectileMovementComponent|SetInitialSpeed (Variables|Default|GetProjectileMovement) (Variables|Default|GetVelocity))
  (switch Utilities|FlowControl|Switch|SwitchonE_Grenades (Variables|Default|GetGrenadeType)
    (:NewEnumerator0
      (Components|StaticMesh|SetStaticMesh _staticmesh "/Game/ReadyOrSwat/BluePrint/CharCreation/Weapons/Grenade_Frag.Grenade_Frag"))
    (:NewEnumerator1
      (Components|StaticMesh|SetStaticMesh _staticmesh "/Game/ReadyOrSwat/BluePrint/CharCreation/Weapons/Grenade_Smoke.Grenade_Smoke"))
    (:NewEnumerator3
      (Components|StaticMesh|SetStaticMesh _staticmesh "/Game/ReadyOrSwat/BluePrint/CharCreation/Weapons/Grenade_Stun.Grenade_Stun"))))
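; Bullet projectile that sets speed, mass and environment damage by caliber, dealing damage through DamageInterFace or radial damage to other hits.
; On bounce, it rolls penetration odds from speed, impact angle and a physical-material data table.
; Recursive backward sphere traces find exits, where a slower replacement bullet spawns, instigated by player 0, losing a flat per-material speed regardless of thickness.
; Ricochets and exits get randomized cone deflection kept off the surface.
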(event OnProjectileBounce(ProjectileMovement)
  (params (ImpactResult :type Hit%20Result%20Structure%20%28by%20ref%29) (ImpactVelocity :type Vector%20%28by%20ref%29 :default "0, 0, 0"))
  (bind (_bblockinghit _binitialoverlap _time _distance _location _impactpoint _normal _impactnormal) (Collision|BreakHitResult ImpactResult))
  (Rendering|Debug|DrawDebugLine (Variables|Default|GetLastPos) _location "(R=1.000000,G=0.095177,B=0.000000,A=1.000000)" 0.0 0.0)
  (Variables|Default|SetLastPos _location)
  (if (CallFunction|ToPenetrate ImpactResult ImpactVelocity)
    (bind (_exitlocation _resultfound _exitnormal) (CallFunction|ComputeExitLocation ImpactResult ImpactVelocity))
    (if _resultfound
      (if (> (CallFunction|GetNewSpeed ImpactResult _exitlocation ImpactVelocity) 0.0)
        (bind _returnvalue (Game|SpawnActorfromClass "Bullet_C" (Math|Transform|MakeTransform _exitlocation) "AlwaysSpawn" 0 (Variables|Default|GetE_BulletType) (Game|GetPlayerCharacter 0)))
        (Variables|/Script/Engine.MovementComponent|SetVelocity (Variables|Bullet_C|GetProjectileMovement _returnvalue) (* ImpactVelocity (/ (CallFunction|GetNewSpeed ImpactResult _exitlocation ImpactVelocity) (Math|Vector|VectorLength ImpactVelocity))))
        (CallFunction|VaryTragect _returnvalue _exitnormal ImpactVelocity _returnvalue)
        (Actor|DestroyActor)
        (else
          (Actor|DestroyActor :!label _label)))
      (else
        (goto _label)))
    (else
      (CallFunction|VaryTragect _impactnormal ImpactVelocity self))))

(event EventTick
  (params (DeltaSeconds :type Float%20%28single-precision%29)))

(event Collision|EventHit
  (params (MyComp :type Primitive%20Component%20Object%20Reference) (Other :type Actor%20Object%20Reference) (OtherComp :type Primitive%20Component%20Object%20Reference) (bSelfMoved :type Boolean) (HitLocation :type Vector :default "0, 0, 0") (HitNormal :type Vector :default "0, 0, 0") (NormalImpulse :type Vector :default "0, 0, 0") (Hit :type Hit%20Result%20Structure%20%28by%20ref%29))
  (bind (_bblockinghit _binitialoverlap _time _distance _location _impactpoint _normal _impactnormal _physmat _hitactor _hitcomponent _hitbonename) (Collision|BreakHitResult Hit))
  (bind _env_damage (Variables|Default|GetENV_Damage))
  (if (Utilities|DoesObjectImplementInterface _hitactor "/Game/ReadyOrSwat/BluePrint/DamageInterFace.DamageInterFace_C")
    (if (not (== (Game|GetInstigator) _hitactor))
      (Class|DamageInterFace|DealDamage(Message) _hitactor (Variables|Default|GetDamage) _hitbonename (Game|GetInstigator))
      (Actor|DestroyActor))
    (else
      (Class|GameplayStatics|ApplyRadialDamagewithFalloff _env_damage _env_damage _impactpoint (Variables|Default|GetENV_MinRadius) (Variables|Default|GetENV_MaxRadius) 1.0 0 0 self (Game|GetInstigatorController) "ECC_Visibility"))))

(event EventBeginPlay
  (Actor|SetLifeSpan 3e+01))

(fn ConstructionScript
  (bind _projectilemovement (Variables|Default|GetProjectileMovement))
  (Variables|Default|SetLastPos (Transformation|GetActorLocation))
  (switch Utilities|FlowControl|Switch|SwitchonE_BulletType (Variables|Default|GetE_BulletType)
    (:NewEnumerator0
      (Variables|/Script/Engine.ProjectileMovementComponent|SetInitialSpeed _projectilemovement 9.22e+03)
      (Variables|Default|SetMass 0.00356)
      (Variables|Default|SetENV_HalfHeight 3e+01)
      (Variables|Default|SetENV_MinRadius 1e+01)
      (Variables|Default|SetENV_MaxRadius 5e+01)
      (Variables|Default|SetENV_Damage 0.05)
      (Variables|Default|SetENV_ImpStrength 25.0))
    (:NewEnumerator1
      (Variables|/Script/Engine.ProjectileMovementComponent|SetInitialSpeed _projectilemovement 8.38e+03)
      (Variables|Default|SetMass 0.01)
      (Variables|Default|SetENV_HalfHeight 1e+02)
      (Variables|Default|SetENV_MinRadius 1e+01)
      (Variables|Default|SetENV_MaxRadius 5e+01)
      (Variables|Default|SetENV_Damage 1.0)
      (Variables|Default|SetENV_ImpStrength 5e+01))
    (:NewEnumerator3
      (Variables|/Script/Engine.ProjectileMovementComponent|SetInitialSpeed _projectilemovement 4.52e+03)
      (Variables|Default|SetMass 0.015)
      (Variables|Default|SetENV_HalfHeight 75.0)
      (Variables|Default|SetENV_MinRadius 1e+01)
      (Variables|Default|SetENV_MaxRadius 5e+01)
      (Variables|Default|SetENV_Damage 0.08)
      (Variables|Default|SetENV_ImpStrength 75.0))
    (:NewEnumerator4
      (Variables|/Script/Engine.ProjectileMovementComponent|SetInitialSpeed _projectilemovement 3.5e+03)
      (Variables|Default|SetMass 0.001)
      (Variables|Default|SetENV_HalfHeight 88.0)
      (Variables|Default|SetENV_MinRadius 1e+01)
      (Variables|Default|SetENV_MaxRadius 5e+01)
      (Variables|Default|SetENV_Damage 15.0)
      (Variables|Default|SetENV_ImpStrength 1e+02))))

(fn ComputeExitLocation
  (params (HitResult :type Hit%20Result%20Structure) (ImpactVelocity :type Vector))
  (bind _returnvalue (Math|Vector|Normalize ImpactVelocity))
  (bind (_bblockinghit _binitialoverlap _time _distance _location _impactpoint _normal _impactnormal _physmat _hitactor) (Collision|BreakHitResult HitResult))
  (bind _array (Utilities|Array|MakeArray "ObjectTypeQuery1" "ObjectTypeQuery2" "ObjectTypeQuery3" "ObjectTypeQuery4" "ObjectTypeQuery6" "ObjectTypeQuery7"))
  (bind (_outhits _returnvalue_2) (Collision|MultiSphereTraceForObjects (+ (* _returnvalue 3e+02) _location) _location (Variables|/Script/Engine.SphereComponent|GetSphereRadius (Variables|Default|GetSphere1)) _array false 0 "None"))
  (if _returnvalue_2
    (for _index (range 0 (Utilities|Array|LastIndex _outhits))
      (if (== (.HitActor (Collision|BreakHitResult (Utilities|Array|Get(acopy) _outhits (- (Utilities|Array|LastIndex _outhits) _index)))) _hitactor)
        (bind (_outhit _returnvalue_3) (Collision|SphereTraceForObjects (+ (.Location (Collision|BreakHitResult (Utilities|Array|Get(acopy) _outhits (- (Utilities|Array|LastIndex _outhits) _index)))) (.ImpactNormal (Collision|BreakHitResult (Utilities|Array|Get(acopy) _outhits (- (Utilities|Array|LastIndex _outhits) _index))))) (+ _returnvalue (+ (.Location (Collision|BreakHitResult (Utilities|Array|Get(acopy) _outhits (- (Utilities|Array|LastIndex _outhits) _index)))) (.ImpactNormal (Collision|BreakHitResult (Utilities|Array|Get(acopy) _outhits (- (Utilities|Array|LastIndex _outhits) _index)))))) (Variables|/Script/Engine.SphereComponent|GetSphereRadius (Variables|Default|GetSphere1)) _array false (Utilities|Array|MakeArray _hitactor) "None"))
        (if _returnvalue_3
          (bind (_exitlocation _resultfound _exitnormal) (CallFunction|ComputeExitLocation _outhit ImpactVelocity))
          (return _exitlocation _resultfound _exitnormal)
          (else
            (return (+ (.Location (Collision|BreakHitResult (Utilities|Array|Get(acopy) _outhits (- (Utilities|Array|LastIndex _outhits) _index)))) (.ImpactNormal (Collision|BreakHitResult (Utilities|Array|Get(acopy) _outhits (- (Utilities|Array|LastIndex _outhits) _index))))) true (.ImpactNormal (Collision|BreakHitResult (Utilities|Array|Get(acopy) _outhits (- (Utilities|Array|LastIndex _outhits) _index))))))))))
  (return "0, 0, 0" false "0, 0, 0"))

(fn GetNewSpeed
  (params (Hit :type Hit%20Result%20Structure) (ExitLocation :type Vector) (ImpactVelcity :type Vector))
  (bind _returnvalue (Utilities|GetDataTableRow "/Game/ReadyOrSwat/BluePrint/PhysMats/BulletPenDataTable.BulletPenDataTable" (Utilities|String|StringToName (Utilities|GetObjectName (.PhysMat (Collision|BreakHitResult Hit)))))
    (:then
      (bind _output_get (LocalVariables|SetJoulesPCM (Utilities|Struct|BreakBullentPenData _returnvalue)))
      (return (- (Math|Vector|VectorLength ImpactVelcity) _output_get)))))

(fn AngleBetweenVectors
  (params (Vec1 :type Vector) (Vec2 :type Vector))
  (return (Class|KismetMathLibrary|DegAcos (Math|Vector|DotProduct (Math|Vector|Normalize Vec1) (Math|Vector|Normalize Vec2)))))

(fn ToPenetrate
  (params (Hit :type Hit%20Result%20Structure) (ImpactVel :type Vector))
  (bind (_bblockinghit _binitialoverlap _time _distance _location _impactpoint _normal _impactnormal _physmat) (Collision|BreakHitResult Hit))
  (bind _returnvalue (Math|Vector|VectorLength ImpactVel))
  (bind _returnvalue_2 (* _impactnormal -1.0))
  (bind _outangle (CallFunction|AngleBetweenVectors ImpactVel _returnvalue_2))
  (bind _returnvalue_3 (Utilities|GetDataTableRow "/Game/ReadyOrSwat/BluePrint/PhysMats/BulletPenDataTable.BulletPenDataTable" (Utilities|String|StringToName (Utilities|GetObjectName _physmat)))
    (:then
      (return (> (* (Math|Float|Clamp(Float) (+ (* _returnvalue (.VelocityGradient (Utilities|Struct|BreakBullentPenData _returnvalue_3))) (.VelocityZInterceot (Utilities|Struct|BreakBullentPenData _returnvalue_3)))) (Math|Float|Clamp(Float) (+ (* (.ImpactAngleGradient (Utilities|Struct|BreakBullentPenData _returnvalue_3)) _outangle) (.InpactAngleZIntercept (Utilities|Struct|BreakBullentPenData _returnvalue_3))))) (Math|Random|RandomFloatinRange 0.0 1.0))))
    (:RowNotFound
      (return (> (* (Math|Float|Clamp(Float) (+ (* 0.0125 _returnvalue) -1.25)) (Math|Float|Clamp(Float) (+ (* -0.022 _outangle) 1.333))) (Math|Random|RandomFloatinRange 0.0 1.0))))))

(fn VaryTragect
  (params (SurfaceNormal :type Vector) (ImpactVelocity :type Vector) (Bullet :type Bullet%20Object%20Reference))
  (bind _projectilemovement (Variables|Bullet_C|GetProjectileMovement Bullet))
  (bind _output_get (LocalVariables|SetInitVar (* (Math|Random|RandomUnitVectorinConeinDegrees (Variables|/Script/Engine.MovementComponent|GetVelocity _projectilemovement) (Math|Float|MapRangeClamped (Math|Vector|VectorLength ImpactVelocity) 3e+03 1e+04 0.0 0.349)) (Math|Vector|VectorLength (Variables|/Script/Engine.MovementComponent|GetVelocity _projectilemovement)))))
  (if (> (CallFunction|AngleBetweenVectors SurfaceNormal _output_get) 89.999001)
    (Variables|/Script/Engine.MovementComponent|SetVelocity _projectilemovement (Math|Vector|RotateVector (LocalVariables|GetInitVar) (* (Math|Rotator|Delta(Rotator) (Math|Rotator|MakeRotfromX SurfaceNormal) (Math|Rotator|MakeRotfromX (LocalVariables|GetInitVar))) (- (/ 89.0 (CallFunction|AngleBetweenVectors SurfaceNormal _output_get)) 1.0))))
    (return)
    (else
      (Variables|/Script/Engine.MovementComponent|SetVelocity _projectilemovement (LocalVariables|GetInitVar))
      (return))))
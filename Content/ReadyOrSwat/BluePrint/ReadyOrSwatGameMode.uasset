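; Game mode for ReadyOrSwat that sets up a local multiplayer match from the player count and difficulty stored in the game instance.
; On BeginPlay it applies the difficulty, enables HBAO, gathers PlayerStarts, then creates each local player and possesses a Player_Chulk at the start tagged with its index plus "Chalk".
; SpawnPlayers similarly possesses RoS_Player pawns at index-tagged starts, but its calls in this event graph are disconnected.
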(event EventBeginPlay
  (bind _asro_sgame_instance (Utilities|Casting|CastToRoSGameInstance (Game|GetGameInstance)))
  (Variables|Default|SetMaxPlayercount (Variables|/Game/ReadyOrSwat/BluePrint/RoSGameInstance.RoSGameInstance_C|GetNoPlayers _asro_sgame_instance))
  (switch string (Variables|/Game/ReadyOrSwat/BluePrint/RoSGameInstance.RoSGameInstance_C|GetDifficulty _asro_sgame_instance)
    (:Default
      (Variables|Default|SetDifficulty "NewEnumerator1" :!label _label))
    (:Rookie
      (Variables|Default|SetDifficulty "NewEnumerator0"))
    (:Normal
      (goto _label))
    (:hard
      (Variables|Default|SetDifficulty "NewEnumerator2"))
    (:INSANE!
      (Variables|Default|SetDifficulty "NewEnumerator3")))
  (Development|ExecuteConsoleCommand "r.hbao.enable = 1" 0)
  (CallFunction|GetPlayerStartPoints)
  (CallFunction|SpawnChalk))

(fn ConstructionScript)

(fn GetPlayerStartPoints
  (bind _outactors (Actor|GetAllActorsOfClass "/Script/Engine.PlayerStart"))
  (Variables|Default|SetPlayerStartArray _outactors))

(fn SpawnPlayers
  (for _index (range 0 (- (Variables|Default|GetMaxPlayercount) 1))
    (bind _output_get (Variables|Default|SetIndex _index))
    (Pawn|UnPossess (Game|GetPlayerController _output_get))
    (for _array_element (Variables|Default|GetPlayerStartArray)
      (if (Utilities|Name|Equal(Name) (Variables|/Script/Engine.PlayerStart|GetPlayerStartTag _array_element) (Utilities|String|StringToName (Utilities|String|ToString(Integer) (Variables|Default|GetIndex))))
        (bind _returnvalue (Game|SpawnActorfromClass "/Game/ReadyOrSwat/BluePrint/RoS_Player.RoS_Player_C" (Transformation|GetActorTransform _array_element) "AlwaysSpawn" 0 (Variables|Default|GetIndex) 0 0))
        (Pawn|Possess (Game|GetPlayerController (Variables|Default|GetIndex)) _returnvalue)
        (Utilities|Array|AddUnique (Variables|Default|GetPlayers) _returnvalue)))))

(fn SpawnChalk
  (for _index (range 0 (- (Variables|Default|GetMaxPlayercount) 1))
    (Variables|Default|SetIndex _index)
    (for _array_element (Variables|Default|GetPlayerStartArray)
      (if (Utilities|Name|Equal(Name) (Variables|/Script/Engine.PlayerStart|GetPlayerStartTag _array_element) (Utilities|String|StringToName (Utilities|String|Append (Utilities|String|ToString(Integer) (Variables|Default|GetIndex)) "Chalk")))
        (bind _returnvalue (Class|GameplayStatics|CreatePlayer (Variables|Default|GetIndex)))
        (Utilities|Array|AddUnique (Variables|Default|GetPlayerControllers) _returnvalue)
        (bind _returnvalue_2 (Game|SpawnActorfromClass "/Game/ReadyOrSwat/BluePrint/Player_Chulk.Player_Chulk_C" (Transformation|GetActorTransform _array_element) "AlwaysSpawn" 0 (Variables|Default|GetIndex) 0))
        (Input|SetInputModeGameOnly (Game|GetPlayerController (Variables|Default|GetIndex)))
        (Pawn|Possess (Game|GetPlayerController (Variables|Default|GetIndex)) _returnvalue_2)))))
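; RoSChar is the Ready or SWAT character, handling guns, health and tactical gear.
; Firing is single or gate-looped automatic, spawning bullets from a constructed weapon object with cone spread on extra projectiles.
; Reload moves rounds from primary or secondary reserves into the magazine.
; Gear functions mostly line-trace from the control rotation for C4, taser stuns, crowbar and door stops; a riot shield attaches, while Sledgehammer is empty.
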(event Custom|AutoFire
  ;[1 1 1] Automatic Fire
  (if (CallFunction|GunIsLoaded?)
    (Utilities|FlowControl|DoOnce false
      (:Completed
        (Utilities|FlowControl|Sequence
          (:then_0
            (goto _label Open))
          (:then_1
            (Utilities|FlowControl|Gate true :!label _label
              (:Exit
                (Variables|WeaponVars|SetIsFireing? true)
                (Math|Integer|IncrementInt (Variables|Default|GetShots)
                  (:%20%20
                    (CallFunction|Shoot)
                    (Utilities|FlowControl|Delay (Variables|/Game/ReadyOrSwat/BluePrint/Inventory/Weapons/WeaponMaster.WeaponMaster_C|GetFireRate (Variables|LoadoutSystem|GetActiveWeaponReferance)))
                    (if (CallFunction|GunIsLoaded?)
                      (goto _label)
                      (else
                        (CallFunction|StopFiring)))))))))))
    (else
      (CallFunction|StopFiring)
      (Development|PrintString (Utilities|String|ToString(Integer) (Variables|WeaponVars|GetAmmoInGun))))))

(event Custom|Shoot
  ;[1 1 1] Fire Projectile
  (CallFunction|RemoveAmmofromMag 1)
  (CallFunction|FireWeapon))

(event Custom|Reload
  ;[1 1 1] Reload
  (if (not (Variables|WeaponVars|GetIsFireing?))
    (Variables|WeaponVars|SetCanSwapWeapn false)
    (if (Variables|WeaponVars|GetIsPrimaryActive?)
      ;;[1 0.00746 0] Primary
      (while (CallFunction|CanReload (Variables|WeaponVars|GetPrimaryAmmo))
        (Variables|WeaponVars|SetAmmoInGun (+ (Variables|WeaponVars|GetAmmoInGun) 1))
        (Variables|WeaponVars|SetPrimaryAmmo (- (Variables|WeaponVars|GetPrimaryAmmo) 1)))
      (Variables|WeaponVars|SetPrimaryAmmoInGun (Variables|WeaponVars|GetAmmoInGun))
      (Variables|WeaponVars|SetCanSwapWeapn true)
      (else
        ;;[0.1494 0 1] Secondary
        (while (CallFunction|CanReload (Variables|WeaponVars|GetSecondaryAmmo))
          (Variables|WeaponVars|SetAmmoInGun (+ (Variables|WeaponVars|GetAmmoInGun) 1))
          (Variables|WeaponVars|SetSecondaryAmmo (- (Variables|WeaponVars|GetSecondaryAmmo) 1)))
        (Variables|WeaponVars|SetSecondaryAmmoInGun (Variables|WeaponVars|GetAmmoInGun))
        (Variables|WeaponVars|SetCanSwapWeapn true)))))

(event Custom|FireGun
  ;[1 1 1] FireWeapon
  (if (Variables|WeaponVars|GetAutoFire?)
    (CallFunction|AutoFire)
    (else
      (CallFunction|SingleFire))))

(event Custom|ConstructWeapon
  (bind _returnvalue (Game|ConstructObjectfromClass (Variables|LoadoutSystem|ClassRefs|GetWeapon_Ref) self))
  (bind _output_get (Variables|LoadoutSystem|SetActiveWeaponReferance _returnvalue))
  (Components|StaticMesh|SetStaticMesh (Variables|Default|GetWeaponMesh) (Variables|/Game/ReadyOrSwat/BluePrint/Inventory/Item_Master.Item_Master_C|GetStaticMeshActor _output_get))
  (Variables|WeaponVars|SetMaxAmmoInGun (Variables|/Game/ReadyOrSwat/BluePrint/Inventory/Weapons/WeaponMaster.WeaponMaster_C|GetMaxAmmoInGun _output_get)))

(event Custom|SingleFire
  ;[1 1 1] SingleFire
  (if (CallFunction|GunIsLoaded?)
    (CallFunction|Shoot)))

(event Custom|StopFiring
  ;[1 1 1] Automatic Fire
  (Utilities|FlowControl|Sequence
    (:then_0
      (Utilities|FlowControl|Gate true) ; enters at Close
    )
    (:then_1
      (Variables|WeaponVars|SetIsFireing? false)
      (Utilities|FlowControl|Delay (Variables|/Game/ReadyOrSwat/BluePrint/Inventory/Weapons/WeaponMaster.WeaponMaster_C|GetFireRate (Variables|LoadoutSystem|GetActiveWeaponReferance)))
      (Utilities|FlowControl|DoOnce false) ; enters at Reset
    )))

(fn ConstructionScript)

(fn GunIsLoaded?
  (if (> (Variables|WeaponVars|GetAmmoInGun) 0)
    (return true)
    (else
      (return false))))

(fn SetHealthValue
  (params (Selection :type E_ArmourType%20Enum :default "NewEnumerator0"))
  (bind _charactermovement (Variables|Character|GetCharacterMovement))
  (switch Utilities|FlowControl|Switch|SwitchonE_ArmourType Selection
    (:NewEnumerator0
      (bind _output_get (Variables|CharacterStatistics|SetHealth_max 2.0))
      (Variables|CharacterStatistics|SetHealth _output_get)
      (bind _output_get_2 (Variables|/Script/Engine.CharacterMovementComponent|SetMaxWalkSpeed _charactermovement 6e+02))
      (Variables|Default|SetMovmentSpeed _output_get_2))
    (:NewEnumerator1
      (bind _output_get_3 (Variables|CharacterStatistics|SetHealth_max 4.0))
      (Variables|CharacterStatistics|SetHealth _output_get_3)
      (bind _output_get_4 (Variables|/Script/Engine.CharacterMovementComponent|SetMaxWalkSpeed _charactermovement 4e+02))
      (Variables|Default|SetMovmentSpeed _output_get_4))))

(fn FTakenDamage
  (params (DamageTaken :type Float%20%28single-precision%29))
  (Development|PrintString (Utilities|String|ToString(Float) DamageTaken))
  (bind _output_get (Variables|CharacterStatistics|SetHealth (- (Variables|CharacterStatistics|GetHealth) DamageTaken)))
  (Development|PrintString (Utilities|String|ToString(Float) (- (Variables|CharacterStatistics|GetHealth) DamageTaken)))
  (return (<= _output_get 0.0)))

(fn HasGear
  (params (GearTypeEnum :type E_GearTypes%20Enum :default "NewEnumerator0") (GearSlot :type Integer))
  (if (or (Utilities|Enum|Equal(Enum) (.GearType (Utilities|GetClassDefaults (Variables|LoadoutSystem|ClassRefs|GetGear1Ref))) GearTypeEnum) (Utilities|Enum|Equal(Enum) GearTypeEnum (.GearType (Utilities|GetClassDefaults (Variables|LoadoutSystem|ClassRefs|GetGear2Ref)))))
    (if (> GearSlot 0)
      (return true)
      (else
        _)))
  (return false))

(fn C4Functions
  (bind _returnvalue (Transformation|GetActorLocation))
  (if (Variables|Gear|GetC4Placed)
    (Default|StartTimer (Variables|Gear|GetPlacedc4Ref))
    (Development|PrintString "Started")
    (Variables|Gear|SetC4Placed false)
    (return false)
    (else
      (bind (_outhit _returnvalue_2) (Collision|LineTraceForObjects _returnvalue (+ _returnvalue (* (Math|Vector|GetForwardVector (Pawn|GetControlRotation :!class /Script/Engine.Pawn)) 5e+02)) (Utilities|Array|MakeArray "ObjectTypeQuery7") false 0 "ForDuration"))
      (if _returnvalue_2
        (bind _returnvalue_3 (Game|SpawnActorfromClass "/Game/ReadyOrSwat/BluePrint/Interabtables/C4Interactable.C4Interactable_C" (Math|Transform|MakeTransform (.Location (Collision|BreakHitResult _outhit)) "0, 0, 0" "1,1,1") "AlwaysSpawn" 0 "50.000000,50.000000,50.000000" 0))
        (Variables|Gear|SetPlacedc4Ref _returnvalue_3)
        (Variables|Gear|SetC4Placed true)
        (return true)
        (else
          (Variables|Gear|SetC4Placed false)
          (return false))))))

(fn RemoveAmmofromMag
  (params (AmmoToRemove :type Integer))
  (bind _output_get (Variables|WeaponVars|SetAmmoInGun (- (Variables|WeaponVars|GetAmmoInGun) AmmoToRemove)))
  (if (Variables|WeaponVars|GetIsPrimaryActive?)
    (Variables|WeaponVars|SetPrimaryAmmoInGun _output_get)
    (else
      (Variables|WeaponVars|SetSecondaryAmmoInGun _output_get)))
  (return))

(fn CanReload
  (params (PorS :type Integer))
  (return (and (<= (Variables|WeaponVars|GetAmmoInGun) (Variables|WeaponVars|GetMaxAmmoInGun)) (> PorS 0))))

(fn AddPrimaryAmmotoBag
  (params (AmmoToAdd :type Integer))
  (Variables|WeaponVars|SetPrimaryAmmo (+ AmmoToAdd (Variables|WeaponVars|GetPrimaryAmmo))))

(fn AddSecondaryAmmotoBag
  (params (AmmoToAdd :type Integer))
  (Variables|WeaponVars|SetSecondaryAmmo (+ AmmoToAdd (Variables|WeaponVars|GetSecondaryAmmo))))

(fn Taser
  (bind _returnvalue (Transformation|GetActorLocation))
  (bind (_outhit _returnvalue_2) (Collision|LineTraceForObjects _returnvalue (+ _returnvalue (* (Math|Vector|GetForwardVector (Pawn|GetControlRotation :!class /Script/Engine.Pawn)) 5e+02)) (Utilities|Array|MakeArray "ObjectTypeQuery3" "ObjectTypeQuery1" "ObjectTypeQuery2" "ObjectTypeQuery7") false (Utilities|Array|MakeArray self) "ForDuration"))
  (if _returnvalue_2
    (bind _asro_schar (Utilities|Casting|CastToRoSChar (.HitActor (Collision|BreakHitResult _outhit))))
    (CallFunction|Tased _asro_schar)
    (Development|PrintString (Utilities|GetDisplayName _asro_schar))))

(fn Crowbar
  (bind _returnvalue (Transformation|GetActorLocation))
  (bind (_outhit _returnvalue_2) (Collision|LineTraceForObjects _returnvalue (+ _returnvalue (* (Math|Vector|GetForwardVector (Pawn|GetControlRotation :!class /Script/Engine.Pawn)) 5e+02)) (Utilities|Array|MakeArray "ObjectTypeQuery1" "ObjectTypeQuery2" "ObjectTypeQuery3" "ObjectTypeQuery7") false 0 "ForDuration"))
  (if _returnvalue_2
    (bind _asdoor (Utilities|Casting|CastToDoor (.HitActor (Collision|BreakHitResult _outhit)))
      (:then
        (Default|Crowbared _asdoor)
        (Development|PrintString "Crowbard")
        (return))
      (:CastFailed
        _)))
  (return))

(fn DoorStop
  (bind _returnvalue (Transformation|GetActorLocation))
  (bind (_outhit _returnvalue_2) (Collision|LineTraceForObjects _returnvalue (+ _returnvalue (* (Math|Vector|GetForwardVector (Pawn|GetControlRotation :!class /Script/Engine.Pawn)) 5e+02)) (Utilities|Array|MakeArray "ObjectTypeQuery1" "ObjectTypeQuery2" "ObjectTypeQuery3" "ObjectTypeQuery7") false 0 "None"))
  (if _returnvalue_2
    (bind _asdoor (Utilities|Casting|CastToDoor (.HitActor (Collision|BreakHitResult _outhit)))
      (:then
        (if (Variables|/Game/ReadyOrSwat/BluePrint/Interabtables/Door.Door_C|GetCrowbared? _asdoor)
          _
          (elif (Variables|/Game/ReadyOrSwat/BluePrint/Interabtables/Door.Door_C|GetHasDoorStop _asdoor)
            (Default|UnlockDoorStop _asdoor)
            (Development|PrintString "Pickedup")
            (return false true)
            (else
              (Default|LockDoorStop _asdoor)
              (Development|PrintString "placed")
              (return true false)))))
      (:CastFailed
        _)))
  (return false false))

(fn Sledgehammer)

(fn Tased
  (Variables|Default|SetMovementDisabled? true)
  (Variables|/Script/Engine.CharacterMovementComponent|SetMaxWalkSpeed (Variables|Character|GetCharacterMovement) 0.0)
  (Utilities|Time|SetTimerbyFunctionName 0 "TasedRecover" 5.0))

(fn TasedRecover
  (Variables|Default|SetMovementDisabled? false)
  (Variables|/Script/Engine.CharacterMovementComponent|SetMaxWalkSpeed (Variables|Character|GetCharacterMovement) 6e+02))

(fn RiotShield
  (bind _returnvalue (Game|SpawnActorfromClass "/Game/ReadyOrSwat/BluePrint/Inventory/Gear/RiotShield_Actor.RiotShield_Actor_C" (Math|Transform|MakeTransform (* (Math|Vector|GetForwardVector (Variables|Default|GetArrow1)) 1e+02) "0, 0, 0" "1,1,1") "AlwaysSpawn" self 0))
  (Transformation|AttachActorToActor _returnvalue self "Arrow1" "KeepRelative" "KeepRelative" "KeepRelative" true))

(fn FireWeapon
  (bind _self self)
  (bind _arrow1 (Variables|Default|GetArrow1))
  (bind _arrow1_2 (Variables|Default|GetArrow1))
  (bind _activeweaponreferance (Variables|LoadoutSystem|GetActiveWeaponReferance))
  (bind _arrow1_3 (Variables|Default|GetArrow1))
  (bind _returnvalue (Transformation|GetWorldLocation _arrow1_2))
  (bind _returnvalue_2 (Transformation|GetWorldTransform _arrow1_3))
  (bind _returnvalue_3 (Transformation|GetWorldLocation _arrow1))
  (bind _e_bullettype (Variables|/Game/ReadyOrSwat/BluePrint/Inventory/Weapons/WeaponMaster.WeaponMaster_C|GetE_BulletType _activeweaponreferance))
  (for _index (range 0 (- (Variables|/Game/ReadyOrSwat/BluePrint/Inventory/Weapons/WeaponMaster.WeaponMaster_C|GetProjectilesToSpawn _activeweaponreferance) 1))
    (if (not (== _index 0))
      (Game|SpawnActorfromClass "/Game/ReadyOrSwat/BluePrint/Bullet.Bullet_C" (Math|Transform|MakeTransform (.location _returnvalue_2) (Math|Rotator|MakeRotfromX (Math|Random|RandomUnitVectorinConeinDegrees (Math|Vector|GetForwardVector (Variables|Default|GetArrow1)) (Variables|/Game/ReadyOrSwat/BluePrint/Inventory/Weapons/WeaponMaster.WeaponMaster_C|GetAccuracy _activeweaponreferance))) (.scale _returnvalue_2)) "AlwaysSpawn" 0 _e_bullettype _self)
      (Effects|SpawnEmitterAttached "/Game/StarterContent/Particles/P_Explosion.P_Explosion" _arrow1 "None" "0, 0, 0" "0, 0, 0" "0.200000,0.200000,0.200000")
      (ForceFeedback|SpawnForceFeedbackatLocation "/Game/ReadyOrSwat/BluePrint/FireWeaponFeedback.FireWeaponFeedback" _returnvalue_3 "0, 0, 0" false 1.0 0.0 0)
      (Audio|PlaySoundatLocation (Variables|/Game/ReadyOrSwat/BluePrint/Inventory/Weapons/WeaponMaster.WeaponMaster_C|GetSoundToPlay (Variables|LoadoutSystem|GetActiveWeaponReferance)) _returnvalue_3 "0, 0, 0" 1.0 1.0 0.0 0 0 0)
      (else
        (Game|SpawnActorfromClass "/Game/ReadyOrSwat/BluePrint/Bullet.Bullet_C" (Transformation|GetWorldTransform _arrow1_3) "AlwaysSpawn" 0 _e_bullettype _self)
        (Effects|SpawnEmitterAttached "/Game/StarterContent/Particles/P_Explosion.P_Explosion" _arrow1_2 "None" "0, 0, 0" "0, 0, 0" "0.200000,0.200000,0.200000")
        (ForceFeedback|SpawnForceFeedbackatLocation "/Game/ReadyOrSwat/BluePrint/FireWeaponFeedback.FireWeaponFeedback" _returnvalue "0, 0, 0" false 1.0 0.0 0)
        (Audio|PlaySoundatLocation (Variables|/Game/ReadyOrSwat/BluePrint/Inventory/Weapons/WeaponMaster.WeaponMaster_C|GetSoundToPlay (Variables|LoadoutSystem|GetActiveWeaponReferance)) _returnvalue "0, 0, 0" 1.0 1.0 0.0 0 0 0)))))

(fn CreateAimBeam
  (params (StartBeamLoc :type Vector) (EndBeamLoc :type Vector))
  (bind _returnvalue (Effects|SpawnEmitteratLocation "/Game/ReadyOrSwat/BluePrint/Interabtables/laster.laster" StartBeamLoc))
  (bind _output_get (Variables|Default|SetLasterBeam _returnvalue))
  (Class|ParticleSystemComponent|SetBeamEndPoint _output_get 0 EndBeamLoc))
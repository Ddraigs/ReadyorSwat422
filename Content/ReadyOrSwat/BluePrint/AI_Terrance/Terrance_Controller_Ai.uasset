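; AI controller for the Terrance enemy that drives its behavior tree and reacts to perception.
; Shortly after BeginPlay it caches the pawn, requests a job from the squad manager and runs BHT_Terrance.
; Sighting the player, unless the state blocks it, enters combat, writes the player to the blackboard and alerts the squad, while hearing switches AI state.
; ReloadAIControlelr pushes a combat order into the blackboard.
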(event OnTargetPerceptionUpdated(AIPerception)
  (params (Actor :type Actor%20Object%20Reference) (Stimulus :type AI%20Stimulus%20Structure))
  (bind _controlledpawnref (Variables|Default|GetControlledPawnRef))
  (bind _controlledpawnref_2 (Variables|Default|GetControlledPawnRef))
  (if (.bSuccessfullySensed (Utilities|Struct|BreakAIStimulus Stimulus))
    (bind _returnvalue (Class|AIPerceptionSystem|GetSenseClassforStimulus Stimulus))
    (if (== _returnvalue "/Script/AIModule.AISense_Sight")
      (bind _asro_s_player (Utilities|Casting|CastToRoS_Player Actor))
      (if (Utilities|Enum|NotEqual(Enum) (Variables|/Game/ReadyOrSwat/BluePrint/AI_Terrance/AI_Terrance.AI_Terrance_C|GetAIState _controlledpawnref) "NewEnumerator7")
        (Variables|/Game/ReadyOrSwat/BluePrint/AI_Terrance/AI_Terrance.AI_Terrance_C|SetAIState _controlledpawnref "NewEnumerator2")
        (Variables|/Game/ReadyOrSwat/BluePrint/AI_Terrance/AI_Terrance.AI_Terrance_C|SetInCombat _controlledpawnref true)
        (Variables|/Game/ReadyOrSwat/BluePrint/AI_Terrance/AI_Terrance.AI_Terrance_C|SetPlayerReferance (Variables|Default|GetControlledPawnRef) _asro_s_player)
        (AI|Components|Blackboard|SetValueasObject (AI|GetBlackboard 0) (Utilities|Name|MakeLiteralName "PlayerReferance") _asro_s_player)
        (Default|AlertSqaud (Variables|/Game/ReadyOrSwat/BluePrint/AI_Terrance/AI_Terrance.AI_Terrance_C|GetSqaudManager _controlledpawnref) (Variables|/Game/ReadyOrSwat/BluePrint/AI_Terrance/AI_Terrance.AI_Terrance_C|GetAISkill _controlledpawnref) (Variables|Default|GetControlledPawnRef)))
      (elif (== _returnvalue "/Script/AIModule.AISense_Hearing")
        (if (or (Utilities|Enum|NotEqual(Enum) (Variables|/Game/ReadyOrSwat/BluePrint/AI_Terrance/AI_Terrance.AI_Terrance_C|GetAIState _controlledpawnref_2) "NewEnumerator2") (Utilities|Enum|NotEqual(Enum) (Variables|/Game/ReadyOrSwat/BluePrint/AI_Terrance/AI_Terrance.AI_Terrance_C|GetAIState _controlledpawnref_2) "NewEnumerator7"))
          (Variables|/Game/ReadyOrSwat/BluePrint/AI_Terrance/AI_Terrance.AI_Terrance_C|SetAIState _controlledpawnref_2 "NewEnumerator5")
          (else
            (Variables|/Game/ReadyOrSwat/BluePrint/AI_Terrance/AI_Terrance.AI_Terrance_C|SetAIState _controlledpawnref_2 "NewEnumerator2")))))))

(event Custom|ReloadAIControlelr
  (params (EnumValue :type Byte))
  (AI|Components|Blackboard|SetValueasEnum (AI|GetBlackboard 0) (Utilities|Name|MakeLiteralName "AICombatOrder") EnumValue))

(event EventBeginPlay
  (Utilities|FlowControl|Delay 0.2)
  (bind _asai_terrance (Utilities|Casting|CastToAI_Terrance (Pawn|GetControlledPawn))
    (:then
      (bind _output_get (Variables|Default|SetControlledPawnRef _asai_terrance))
      (Default|GetJob (Variables|/Game/ReadyOrSwat/BluePrint/AI_Terrance/AI_Terrance.AI_Terrance_C|GetSqaudManager _output_get) _output_get)
      (AI|RunBehaviorTree "/Game/ReadyOrSwat/BluePrint/AI_Terrance/BHT_Terrance.BHT_Terrance"))
    (:CastFailed
      (Development|PrintString "Hello"))))

(fn ConstructionScript)
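; Behavior tree service for the AI_Terrance enemy or squad AI that syncs pawn state into the blackboard.
; Each AI tick casts the controlled pawn to AI_Terrance and copies its AIState, AICombatOrder and player reference into blackboard keys.
; A failed cast prints a debug error string instead.
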(event EventReceiveTickAI
  (params (OwnerController :type AI%20Controller%20Object%20Reference) (ControlledPawn :type Pawn%20Object%20Reference) (DeltaSeconds :type Float%20%28single-precision%29))
  (bind _asai_terrance (Utilities|Casting|CastToAI_Terrance ControlledPawn)
    (:then
      (Class|BTFunctionLibrary|SetBlackboardValueasEnum (Variables|Default|GetAiStateBB) (Variables|/Game/ReadyOrSwat/BluePrint/AI_Terrance/AI_Terrance.AI_Terrance_C|GetAIState _asai_terrance))
      (Class|BTFunctionLibrary|SetBlackboardValueasEnum (Variables|Default|GetAICombatOrder) (Variables|/Game/ReadyOrSwat/BluePrint/AI_Terrance/AI_Terrance.AI_Terrance_C|GetAI_CombatOrder _asai_terrance))
      (Class|BTFunctionLibrary|SetBlackboardValueasObject (Variables|Default|GetPlayerReferance) (Variables|/Game/ReadyOrSwat/BluePrint/AI_Terrance/AI_Terrance.AI_Terrance_C|GetPlayerReferance _asai_terrance)))
    (:CastFailed
      (Development|PrintString "Gone Done fucked up the AIStatechange service"))))
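; Behavior tree task for the Terrance AI that checks whether a chosen cover destination is still valid.
; It runs a 200-unit pawn sphere overlap, filtered to RoS_Player, around the move-to location read from the blackboard.
; A player inside that radius sets the IsCoverVaild blackboard bool false, otherwise true, and the task then finishes successfully.
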(event EventReceiveExecuteAI
  (params (OwnerController :type AI%20Controller%20Object%20Reference) (ControlledPawn :type Pawn%20Object%20Reference))
  (bind (_outactors _returnvalue) (Collision|SphereOverlapActors (Class|BTFunctionLibrary|GetBlackboardValueasVector (Variables|Default|GetBB_MoveToLoc)) 2e+02 (Utilities|Array|MakeArray "ObjectTypeQuery3") "/Game/ReadyOrSwat/BluePrint/RoS_Player.RoS_Player_C"))
  (if _returnvalue
    (for _array_element _outactors
      (Utilities|Casting|CastToRoS_Player _array_element)
      (Class|BTFunctionLibrary|SetBlackboardValueasBool (Variables|Default|GetIsCoverVaild) false))
    (else
      (Class|BTFunctionLibrary|SetBlackboardValueasBool (Variables|Default|GetIsCoverVaild) true)))
  (AI|BehaviorTree|FinishExecute true))
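; Behavior tree task that gives AI_Terrance a random destination around the player, so the AI can surround them.
; It picks a random point inside the player's BoxAroundPlayer extents, centred on the player's location, and writes it to the BBMoveTo blackboard key.
; It uses the pawn's cached player reference, or the first RoS_Player in the world when that is invalid, then finishes successfully.
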(event EventReceiveExecuteAI
  (params (OwnerController :type AI%20Controller%20Object%20Reference) (ControlledPawn :type Pawn%20Object%20Reference))
  (bind _asai_terrance (Utilities|Casting|CastToAI_Terrance ControlledPawn))
  (Utilities|IsValid (Variables|/Game/ReadyOrSwat/BluePrint/AI_Terrance/AI_Terrance.AI_Terrance_C|GetPlayerReferance _asai_terrance)
    (:Is%20Valid
      (AI|BehaviorTree|SetBlackboardValueasVector (Variables|Default|GetBB_MoveTo) (Math|Random|RandomPointinBoundingBox (Transformation|GetActorLocation (Variables|/Game/ReadyOrSwat/BluePrint/AI_Terrance/AI_Terrance.AI_Terrance_C|GetPlayerReferance _asai_terrance)) (Components|Box|GetScaledBoxExtent (Variables|/Game/ReadyOrSwat/BluePrint/RoS_Player.RoS_Player_C|GetBoxAroundPlayer (Variables|/Game/ReadyOrSwat/BluePrint/AI_Terrance/AI_Terrance.AI_Terrance_C|GetPlayerReferance _asai_terrance))))))
    (:Is%20Not%20Valid
      (bind _outactors (Actor|GetAllActorsOfClass "/Game/ReadyOrSwat/BluePrint/RoS_Player.RoS_Player_C"))
      (AI|BehaviorTree|SetBlackboardValueasVector (Variables|Default|GetBB_MoveTo) (Math|Random|RandomPointinBoundingBox (Transformation|GetActorLocation (Utilities|Array|Get(acopy) _outactors)) (Components|Box|GetScaledBoxExtent (Variables|/Game/ReadyOrSwat/BluePrint/RoS_Player.RoS_Player_C|GetBoxAroundPlayer (Utilities|Array|Get(acopy) _outactors)))))))
  (AI|BehaviorTree|FinishExecute true))
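; Squad manager that spawns and coordinates AI_Terrance enemies for standard or high-value-target (HVT) squads.
; Members spawn randomly within a spawn point's box in skill tiers, register with the manager and update mission remaining counters (only the HVT in HVT squads).
; Skill sets each member's job and whether alerts reach the whole squad or only nearby allies.
; Orders depend on morale, ammo and skill, handling only assault rifles; surround logic is disconnected.
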(event Custom|AlertSqaud
  (params (Skill :type Integer) (TerranceReferance :type AI%20Terrance%20Object%20Reference))
  (if (> Skill 33)
    (Variables|Default|SetPlayerDetected true)
    (for _array_element (Variables|Default|GetSqaudArray)
      (Utilities|IsValid _array_element
        (:Is%20Valid
          (if (Utilities|Enum|NotEqual(Enum) (Variables|/Game/ReadyOrSwat/BluePrint/AI_Terrance/AI_Terrance.AI_Terrance_C|GetAIState _array_element) "NewEnumerator7")
            (Variables|/Game/ReadyOrSwat/BluePrint/AI_Terrance/AI_Terrance.AI_Terrance_C|SetAIState _array_element "NewEnumerator2")))))
    (else
      (bind _outactors (Collision|SphereOverlapActors (Transformation|GetActorLocation TerranceReferance) 2.5e+02 (Utilities|Array|MakeArray "ObjectTypeQuery3") "/Game/ReadyOrSwat/BluePrint/AI_Terrance/AI_Terrance.AI_Terrance_C"))
      (for _array_element_2 _outactors
        (bind _asai_terrance (Utilities|Casting|CastToAI_Terrance _array_element_2))
        (Utilities|IsValid _asai_terrance
          (:Is%20Valid
            (if (Utilities|Enum|NotEqual(Enum) (Variables|/Game/ReadyOrSwat/BluePrint/AI_Terrance/AI_Terrance.AI_Terrance_C|GetAIState _asai_terrance) "NewEnumerator7")
              (Variables|/Game/ReadyOrSwat/BluePrint/AI_Terrance/AI_Terrance.AI_Terrance_C|SetAIState _asai_terrance "NewEnumerator2"))))))))

(event Custom|GetJob
  (params (Terrance :type AI%20Terrance%20Object%20Reference))
  (bind _aiskill (Variables|/Game/ReadyOrSwat/BluePrint/AI_Terrance/AI_Terrance.AI_Terrance_C|GetAISkill Terrance))
  (if (< _aiskill 33)
    (Variables|/Game/ReadyOrSwat/BluePrint/AI_Terrance/AI_Terrance.AI_Terrance_C|SetAIState Terrance "NewEnumerator0")
    (elif (< _aiskill 66)
      (Variables|/Game/ReadyOrSwat/BluePrint/AI_Terrance/AI_Terrance.AI_Terrance_C|SetAIState Terrance "NewEnumerator1")
      (else
        (if (> _aiskill 65)
          _
          (else
            _))
        (Variables|/Game/ReadyOrSwat/BluePrint/AI_Terrance/AI_Terrance.AI_Terrance_C|SetAIState Terrance "NewEnumerator6")))))

(event Custom|GiveAnOrder
  (params (Terrance :type AI%20Terrance%20Object%20Reference))
  (CallFunction|OrdertoGive Terrance))

(event Custom|CreateStandardSqaud
  ;[1 0 0] Remove Later
  (bind _asready_or_swat_game_mode (Utilities|Casting|CastToReadyOrSwatGameMode (Game|GetGameMode)))
  (Variables|Default|SetGameModeRef _asready_or_swat_game_mode)
  (CallFunction|SpawnAI))

(event Custom|CreateHVTSquad
  (bind _asready_or_swat_game_mode (Utilities|Casting|CastToReadyOrSwatGameMode (Game|GetGameMode)))
  (Variables|Default|SetGameModeRef _asready_or_swat_game_mode)
  (CallFunction|SpawnHVTAI))

(event EventBeginPlay)

(fn ConstructionScript)

(fn GetSpawnTransform
  (params (Spawnpoint :type Spawn%20Point%20Object%20Reference))
  (bind _returnvalue (Transformation|GetActorLocation Spawnpoint))
  (bind _box (Variables|/Game/ReadyOrSwat/BluePrint/Tasks/SpawnPoint.SpawnPoint_C|GetBox Spawnpoint))
  (bind _returnvalue_2 (Components|Box|GetScaledBoxExtent _box))
  (bind _returnvalue_3 (Math|Random|RandomPointinBoundingBox _returnvalue _returnvalue_2))
  (return (Math|Transform|MakeTransform (Math|Vector|MakeVector (.x _returnvalue_3) (.y _returnvalue_3) (.Z (Math|Vector|BreakVector _returnvalue))))))

(fn AISkill
  (return (Math|Integer|Clamp(Integer) (Math|Random|RandomInteger 101) 0 100)))

(fn OrdertoGive
  (params (InputPin :type AI%20Terrance%20Object%20Reference))
  (if (> (Variables|/Game/ReadyOrSwat/BluePrint/AI_Terrance/AI_Terrance.AI_Terrance_C|GetAiMoral InputPin) (Math|Conversions|ToFloat(Integer) (Variables|/Game/ReadyOrSwat/BluePrint/AI_Terrance/AI_Terrance.AI_Terrance_C|GetAISkill InputPin)))
    (if (Variables|/Game/ReadyOrSwat/BluePrint/AI_Terrance/AI_Terrance.AI_Terrance_C|GetHasAmmo? InputPin)
      (switch Utilities|FlowControl|Switch|SwitchonAI_Weapon (Variables|/Game/ReadyOrSwat/BluePrint/AI_Terrance/AI_Terrance.AI_Terrance_C|GetE_Weapon InputPin)
        (:NewEnumerator0
          (if (< (Variables|/Game/ReadyOrSwat/BluePrint/AI_Terrance/AI_Terrance.AI_Terrance_C|GetAISkill InputPin) 33)
            (bind _output_get (Variables|/Game/ReadyOrSwat/BluePrint/AI_Terrance/AI_Terrance.AI_Terrance_C|SetAI_CombatOrder InputPin "NewEnumerator2"))
            (return "NewEnumerator2" _output_get)
            (else
              (bind _output_get_2 (Variables|/Game/ReadyOrSwat/BluePrint/AI_Terrance/AI_Terrance.AI_Terrance_C|SetAI_CombatOrder InputPin "NewEnumerator3"))
              (return "NewEnumerator2" _output_get_2)))))
      (else
        (bind _output_get_3 (Variables|/Game/ReadyOrSwat/BluePrint/AI_Terrance/AI_Terrance.AI_Terrance_C|SetAI_CombatOrder InputPin "NewEnumerator4"))
        (return "NewEnumerator2" _output_get_3)))
    (else
      (bind _output_get_4 (Variables|/Game/ReadyOrSwat/BluePrint/AI_Terrance/AI_Terrance.AI_Terrance_C|SetAIState InputPin "NewEnumerator3"))
      (return _output_get_4 "NewEnumerator3"))))

(fn SurroundCheck
  (params (TerranceArray :type AI%20Terrance%20Object%20Reference) (AITerrance_NONArray :type AI%20Terrance%20Object%20Reference))
  (bind _e_weapon (Variables|/Game/ReadyOrSwat/BluePrint/AI_Terrance/AI_Terrance.AI_Terrance_C|GetE_Weapon TerranceArray))
  (return (Math|Boolean|ANDBoolean (Variables|/Game/ReadyOrSwat/BluePrint/AI_Terrance/AI_Terrance.AI_Terrance_C|GetHasAmmo? TerranceArray) (Utilities|Enum|Equal(Enum) (Variables|/Game/ReadyOrSwat/BluePrint/AI_Terrance/AI_Terrance.AI_Terrance_C|GetAI_CombatOrder TerranceArray) "NewEnumerator0") (< (Variables|/Game/ReadyOrSwat/BluePrint/AI_Terrance/AI_Terrance.AI_Terrance_C|GetAISkill TerranceArray) (Variables|/Game/ReadyOrSwat/BluePrint/AI_Terrance/AI_Terrance.AI_Terrance_C|GetAISkill AITerrance_NONArray)) (or (Utilities|Enum|NotEqual(Enum) _e_weapon "NewEnumerator2") (Utilities|Enum|NotEqual(Enum) _e_weapon "NewEnumerator3")))))

(fn GetTarget
  (bind _outactors (Actor|GetAllActorsOfClass "/Game/ReadyOrSwat/BluePrint/RoS_Player.RoS_Player_C"))
  (return (Utilities|Array|Get(acopy) _outactors (- (Variables|/Game/ReadyOrSwat/BluePrint/ReadyOrSwatGameMode.ReadyOrSwatGameMode_C|GetMaxPlayercount (Variables|Default|GetGameModeRef)) 1))))

(fn SquadSpawnFunc
  (params (Spawnpoint :type Spawn%20Point%20Object%20Reference) (AISkill :type Integer))
  (bind _returnvalue (Game|SpawnActorfromClass "/Game/ReadyOrSwat/BluePrint/AI_Terrance/AI_Terrance.AI_Terrance_C" (CallFunction|GetSpawnTransform Spawnpoint) "AdjustIfPossibleButAlwaysSpawn" 0 AISkill "NewEnumerator0" false 0))
  (return _returnvalue))

(fn SpawnAI
  (bind _outactors (Actor|GetAllActorsOfClass "/Game/ReadyOrSwat/BluePrint/Tasks/SpawnPoint.SpawnPoint_C"))
  (for _index (range 0 (Math|Integer|Clamp(Integer) (- (- (Variables|Default|GetSquadSizes) 1) 4) 4 8))
    (bind _returnvalue (CallFunction|SquadSpawnFunc (Utilities|Array|Get(acopy) _outactors (Variables|Default|GetSpawnPointIndex)) (Math|Random|RandomIntegerinRange 1 33)))
    (Utilities|Array|AddUnique (Variables|Default|GetSqaudArray) _returnvalue)
    (Variables|/Game/ReadyOrSwat/BluePrint/AI_Terrance/AI_Terrance.AI_Terrance_C|SetSqaudManager _returnvalue self)
    (Math|Integer|IncrementInt (Variables|/Game/ReadyOrSwat/BluePrint/Tasks/MissionGen.MissionGen_C|GetTerryRemaining (Variables|Default|GetMissionGenSysRef))))
  (for _index_2 (range 0 (Math|Integer|Clamp(Integer) (- (- (Variables|Default|GetSquadSizes) 1) 5) 3 6))
    (bind _returnvalue_2 (CallFunction|SquadSpawnFunc (Utilities|Array|Get(acopy) _outactors (Variables|Default|GetSpawnPointIndex)) (Math|Random|RandomIntegerinRange 34 66)))
    (Utilities|Array|AddUnique (Variables|Default|GetSqaudArray) _returnvalue_2)
    (Variables|/Game/ReadyOrSwat/BluePrint/AI_Terrance/AI_Terrance.AI_Terrance_C|SetSqaudManager _returnvalue_2 self)
    (Math|Integer|IncrementInt (Variables|/Game/ReadyOrSwat/BluePrint/Tasks/MissionGen.MissionGen_C|GetTerryRemaining (Variables|Default|GetMissionGenSysRef))))
  (for _index_3 (range 0 (Math|Integer|Clamp(Integer) (- (- (Variables|Default|GetSquadSizes) 1) 5) 1 2))
    (bind _returnvalue_3 (CallFunction|SquadSpawnFunc (Utilities|Array|Get(acopy) _outactors (Variables|Default|GetSpawnPointIndex)) (Math|Random|RandomIntegerinRange 66 100)))
    (Utilities|Array|AddUnique (Variables|Default|GetSqaudArray) _returnvalue_3)
    (Variables|/Game/ReadyOrSwat/BluePrint/AI_Terrance/AI_Terrance.AI_Terrance_C|SetSqaudManager _returnvalue_3 self)
    (Math|Integer|IncrementInt (Variables|/Game/ReadyOrSwat/BluePrint/Tasks/MissionGen.MissionGen_C|GetTerryRemaining (Variables|Default|GetMissionGenSysRef))))
  (bind _outactors_2 (Actor|GetAllActorsOfClass "/Game/ReadyOrSwat/BluePrint/RoS_Player.RoS_Player_C"))
  (Variables|Default|SetPlayerRefs _outactors_2))

(fn SpawnHVTAI
  (bind _outactors (Actor|GetAllActorsOfClass "/Game/ReadyOrSwat/BluePrint/Tasks/SpawnPoint.SpawnPoint_C"))
  (for _index (range 0 (Math|Integer|Clamp(Integer) (- (- (Variables|Default|GetSquadSizes) 1) 4) 4 8))
    (bind _returnvalue (CallFunction|SquadSpawnFunc (Utilities|Array|Get(acopy) _outactors (Variables|Default|GetSpawnPointIndex)) (Math|Random|RandomIntegerinRange 1 33)))
    (Utilities|Array|AddUnique (Variables|Default|GetSqaudArray) _returnvalue)
    (Variables|/Game/ReadyOrSwat/BluePrint/AI_Terrance/AI_Terrance.AI_Terrance_C|SetSqaudManager _returnvalue self))
  (for _index_2 (range 0 (Math|Integer|Clamp(Integer) (- (- (Variables|Default|GetSquadSizes) 1) 5) 3 6))
    (bind _returnvalue_2 (CallFunction|SquadSpawnFunc (Utilities|Array|Get(acopy) _outactors (Variables|Default|GetSpawnPointIndex)) (Math|Random|RandomIntegerinRange 34 66)))
    (Utilities|Array|AddUnique (Variables|Default|GetSqaudArray) _returnvalue_2)
    (Variables|/Game/ReadyOrSwat/BluePrint/AI_Terrance/AI_Terrance.AI_Terrance_C|SetSqaudManager _returnvalue_2 self))
  (bind _returnvalue_3 (Game|SpawnActorfromClass "/Game/ReadyOrSwat/BluePrint/AI_Terrance/AI_Terrance.AI_Terrance_C" (CallFunction|GetSpawnTransform (Utilities|Array|Get(acopy) _outactors (Variables|Default|GetSpawnPointIndex))) "AdjustIfPossibleButAlwaysSpawn" 0 99 "NewEnumerator0" true 0))
  (Utilities|Array|AddUnique (Variables|Default|GetSqaudArray) _returnvalue_3)
  (Variables|/Game/ReadyOrSwat/BluePrint/AI_Terrance/AI_Terrance.AI_Terrance_C|SetSqaudManager _returnvalue_3 self)
  (Math|Integer|IncrementInt (Variables|/Game/ReadyOrSwat/BluePrint/Tasks/MissionGen.MissionGen_C|GetHVTRemaining (Variables|Default|GetMissionGenSysRef))
    (:%20%20
      (bind _outactors_2 (Actor|GetAllActorsOfClass "/Game/ReadyOrSwat/BluePrint/RoS_Player.RoS_Player_C"))
      (Variables|Default|SetPlayerRefs _outactors_2))))
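; Enemy AI character for Ready or Swat that fights the player and can surrender or be killed, updating MissionGen and player tallies.
; Timer-driven rifle bursts check arc and range, spawn bullets in skill-based cones, then require a montage reload.
; Morale drops from damage, nearby bullets and yells, recovers near allies, and triggers surrender when depleted.
; Only the assault rifle has firing logic; squad orders come from SqaudManager, and death ragdolls the body before destroying it.
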(event OnComponentBeginOverlap(Box)
  (params (OverlappedComponent :type Primitive%20Component%20Object%20Reference) (OtherActor :type Actor%20Object%20Reference) (OtherComp :type Primitive%20Component%20Object%20Reference) (OtherBodyIndex :type Integer) (bFromSweep :type Boolean) (SweepResult :type Hit%20Result%20Structure%20%28by%20ref%29))
  (Utilities|Casting|CastToAI_Terrance OtherActor
    (:then
      (Math|Float|IncrementFloat (Variables|Default|GetAllysAround)))
    (:CastFailed
      (bind _asbullet (Utilities|Casting|CastToBullet OtherActor))
      (bind _output_get (Variables|Default|SetAiMoral (- (Variables|Default|GetAiMoral) (CallFunction|AISkillBulletFear))))
      (bind _asro_s_player (Utilities|Casting|CastToRoS_Player (Game|GetInstigator _asbullet)))
      (Variables|Default|SetPlayerReferance _asro_s_player)
      (Development|PrintString (Utilities|String|ToString(Float) _output_get)))))

(event OnComponentEndOverlap(Box)
  (params (OverlappedComponent :type Primitive%20Component%20Object%20Reference) (OtherActor :type Actor%20Object%20Reference) (OtherComp :type Primitive%20Component%20Object%20Reference) (OtherBodyIndex :type Integer))
  (Utilities|Casting|CastToAI_Terrance OtherActor)
  (Math|Float|DecrementFloat (Variables|Default|GetAllysAround)))

(event Custom|GetAnOrder
  ;[1 1 1] Gets  ZEE order
  (Default|GiveAnOrder (Variables|Default|GetSqaudManager) self))

(event Custom|Shoot
  ;[1 1 1] StartShootCommad
  (if (not (Variables|Default|GetDead?))
    (if (and (Variables|Default|GetHasAmmo?) (not (Variables|Default|GetIsReloading)))
      (Variables|Default|SetFiring? true)
      (Variables|Default|SetIsAiming true)
      (switch Utilities|FlowControl|Switch|SwitchonAI_Weapon (Variables|Default|GetE_Weapon)
        (:NewEnumerator0
          (CallFunction|Assulterifle)))
      (else
        (Variables|Default|SetIsAiming false)
        (Variables|Default|SetFiring? false)
        (Variables|Default|SetAI_CombatOrder "NewEnumerator4")
        (CallFunction|Reload)))))

(event Custom|Reload
  ;[1 1 1] Reload
  (if (not (Variables|Default|GetIsReloading))
    (Animation|Montage|PlayMontage (Variables|Character|GetMesh) "/Game/ReadyOrSwat/Animation/Reload_Crouching_Montage.Reload_Crouching_Montage"
      (:then
        (Variables|Default|SetIsReloading true))
      (:OnCompleted
        (Variables|Default|SetHasAmmo? true)
        (Variables|Default|SetIsReloading false)
        (Variables|Default|SetShotsFired 0)))))

(event Custom|Assulterifle
  ;[1 1 1] AssultRifle
  (Variables|Default|SetIsAiming true)
  (Variables|Default|SetBurstFire (Math|Random|RandomIntegerinRange 4 10))
  (bind _returnvalue (Utilities|Time|SetTimerbyEvent (delegate Custom|Burst) 0.8 true))
  (Variables|Default|SetRifleTimmer _returnvalue))

(event Custom|Burst
  (bind _arrow1 (Variables|Default|GetArrow1))
  (bind _returnvalue (Transformation|GetWorldLocation _arrow1))
  ;[1 1 1] AssultRifle
  (if (and (<= (Variables|Default|GetShotsFired) (Variables|Default|GetBurstFire)) (not (Variables|Default|GetDead?)))
    (if (CallFunction|FrontFiringAcr)
      (Utilities|FlowControl|Delay 0.5)
      (Variables|Default|SetFiring? true)
      (Math|Integer|IncrementInt (Variables|Default|GetShotsFired)
        (:%20%20
          (Game|SpawnActorfromClass "/Game/ReadyOrSwat/BluePrint/Bullet.Bullet_C" (CallFunction|BulletSpawnTransform) "Undefined" 0 "NewEnumerator1" 0)
          (Effects|SpawnEmitteratLocation "/Game/StarterContent/Particles/P_Explosion.P_Explosion" _returnvalue "0, 0, 0" "0.200000,0.200000,0.200000")
          (Audio|PlaySoundatLocation "/Game/ReadyOrSwat/BluePrint/Inventory/Weapons/Sounds/M4A1Shot_TomFix.M4A1Shot_TomFix" _returnvalue "0, 0, 0" 1.0 1.0 0.0 0 0 0)))
      (else
        (Variables|Default|SetFiring? false)
        (bind _result (Math|Integer|IncrementInt (Variables|Default|GetNoShot))
          (:%20%20
            (if (> _result 4)
              (Variables|Default|SetIsAiming false)
              (CallFunction|StopShooting))))))
    (else
      (Variables|Default|SetFiring? false)
      (Variables|Default|SetIsAiming false)
      (Variables|Default|SetHasAmmo? false))))

(event Custom|StopShooting
  ;[1 1 1] StopShooting
  (Utilities|Time|ClearandInvalidateTimerbyHandle (Variables|Default|GetRifleTimmer))
  (Variables|Default|SetFiring? false)
  (Variables|Default|SetIsAiming false))

(event Custom|MoraleDamage
  (params (Float :type Float%20%28single-precision%29) (IsYell? :type Boolean) (PlayerReferance :type Ro%20S%20Player%20Object%20Reference))
  (if IsYell?
    (if (Variables|Default|GetHasBeenTelledAT)
      _
      (else
        (Variables|Default|SetHasBeenTelledAT true)
        (bind _output_get (Variables|Default|SetAiMoral (- (Variables|Default|GetAiMoral) (- Float (Math|Conversions|ToFloat(Integer) (Variables|Default|GetAISkill)))) :!label _label))))
    (else
      (goto _label)))
  (Development|PrintString (Utilities|String|ToString(Float) _output_get))
  (Animation|Montage|PlayMontage (Variables|Character|GetMesh) "/Game/ReadyOrSwat/Animation/Hit_Reaction_Montage.Hit_Reaction_Montage"
    (:then
      (Variables|Default|SetPlayerReferance PlayerReferance))
    (:OnCompleted
      (Utilities|FlowControl|RetriggerableDelay 5e+01)
      (Variables|Default|SetHasBeenTelledAT false))))

(event EventDealDamage
  (params (Damage :type Float%20%28single-precision%29) (HitBoneName :type Name :default "None") (DamageInstergater :type Actor%20Object%20Reference))
  ;[1 1 1] Damage and death
  (Variables|Default|SetAiMoral (Math|Float|Clamp(Float) (- (Variables|Default|GetAiMoral) 3.0) 0.0 1e+02))
  (bind _output_get (Variables|Default|SetHealth (- (Variables|Default|GetHealth) Damage)))
  (if (<= _output_get 0.0)
    (Variables|Default|SetDead? true)
    (bind _asro_s_player (Utilities|Casting|CastToRoS_Player DamageInstergater))
    (Utilities|FlowControl|Sequence
      (:then_0
        (Utilities|FlowControl|DoOnce false
          (:Completed
            (Math|Integer|IncrementInt (Variables|/Game/ReadyOrSwat/BluePrint/RoS_Player.RoS_Player_C|GetPlayerKills _asro_s_player)
              (:%20%20
                (if (Variables|Default|GetSurrendered)
                  (Math|Integer|DecrementInt (Variables|/Game/ReadyOrSwat/BluePrint/RoS_Player.RoS_Player_C|GetPlayerPacified _asro_s_player))
                  (else
                    (bind _outactors (Actor|GetAllActorsOfClass "/Game/ReadyOrSwat/BluePrint/Tasks/MissionGen.MissionGen_C"))
                    (if (Variables|Default|GetIsHVT)
                      (Math|Integer|DecrementInt (Variables|/Game/ReadyOrSwat/BluePrint/Tasks/MissionGen.MissionGen_C|GetHVTRemaining (Utilities|Array|Get(acopy) _outactors)))
                      (else
                        (Math|Integer|DecrementInt (Variables|/Game/ReadyOrSwat/BluePrint/Tasks/MissionGen.MissionGen_C|GetTerryRemaining (Utilities|Array|Get(acopy) _outactors))))))))))))
      (:then_1
        (Physics|SetSimulatePhysics (Variables|Character|GetMesh) true)
        (Collision|SetCollisionEnabled (Variables|Character|GetMesh) "QueryAndPhysics")
        (Collision|SetCollisionEnabled (Variables|Collision|GetCapsuleComponent) "NoCollision")
        (Utilities|FlowControl|Delay 1e+01)
        (Actor|DestroyActor)))
    (else
      (Variables|Default|SetDead? false))))

(event EventIsCoverAvilable
  (params (IsCoverAvliable :type Boolean) (CoverRot :type Rotator :default "0, 0, 0"))
  (Variables|Default|SetCoverAvilable IsCoverAvliable)
  (Variables|Default|SetCoverRot CoverRot))

(event EventBeginPlay
  ;[1 1 1] Event Begin play
  (Utilities|FlowControl|Delay 0.2)
  (Utilities|Time|SetTimerbyFunctionName self "MoralTimer" 3.0 true)
  (bind _asterrance_controller_ai (Utilities|Casting|CastToTerrance_Controller_Ai (AI|GetAIController self)))
  (Variables|Default|SetAI_Controller _asterrance_controller_ai)
  (bind _outactors (Actor|GetAllActorsOfClass "/Game/ReadyOrSwat/BluePrint/RoS_Player.RoS_Player_C"))
  (Variables|Default|SetPlayerReferance (Utilities|Array|Get(acopy) _outactors))
  (Rendering|SetVisibility (Variables|Default|GetBillboard) (Variables|Default|GetIsHVT) false))

(fn ConstructionScript
  (bind _staticmesh (Variables|Default|GetStaticMesh))
  (switch Utilities|FlowControl|Switch|SwitchonAI_Weapon (Variables|Default|GetE_Weapon)
    (:NewEnumerator0
      (Components|StaticMesh|SetStaticMesh _staticmesh "/Game/ReadyOrSwat/BluePrint/CharCreation/Weapons/M4A1.M4A1"))
    (:NewEnumerator1
      (Components|StaticMesh|SetStaticMesh _staticmesh "/Game/ReadyOrSwat/BluePrint/CharCreation/Weapons/M4A1.M4A1"))
    (:NewEnumerator2
      (Components|StaticMesh|SetStaticMesh _staticmesh "/Game/ReadyOrSwat/BluePrint/CharCreation/Weapons/M4A1.M4A1"))
    (:NewEnumerator3
      (Components|StaticMesh|SetStaticMesh _staticmesh "/Game/ReadyOrSwat/BluePrint/CharCreation/Weapons/M4A1.M4A1"))
    (:NewEnumerator4
      (Components|StaticMesh|SetStaticMesh _staticmesh "/Game/ReadyOrSwat/BluePrint/CharCreation/Weapons/M9_Mag_Box001.M9_Mag_Box001"))))

(fn MoralTimer
  (if (> (Variables|Default|GetAiMoral) 0.0)
    (if (> (Variables|Default|GetAllysAround) 1.0)
      (Variables|Default|SetAiMoral (Math|Float|Clamp(Float) (+ (Variables|Default|GetAiMoral) (/ (Variables|Default|GetAllysAround) 1e+01)) 0.0 1e+02))
      (return)
      (else
        _))
    (else
      (CallFunction|Surrender)))
  (return))

(fn IsTakeingCover
  (params (IsTakingCover :type Boolean))
  (if (not (Variables|Default|GetIsAiming))
    (bind _output_get (Variables|Default|SetIsTakingCover IsTakingCover))
    (if _output_get
      (Transformation|SetActorRotation (Variables|Default|GetCoverRot)))
    (else
      (Variables|Default|SetIsTakingCover false))))

(fn Surrender
  (if (Variables|Default|GetDead?)
    _
    (elif (Variables|Default|GetSurrendered)
      _
      (else
        (Variables|Default|SetAIState "NewEnumerator7")
        (Variables|Default|SetSurrendered true)
        (bind _outactors (Actor|GetAllActorsOfClass "/Game/ReadyOrSwat/BluePrint/Tasks/MissionGen.MissionGen_C"))
        (if (Variables|Default|GetIsHVT)
          (Math|Integer|DecrementInt (Variables|/Game/ReadyOrSwat/BluePrint/Tasks/MissionGen.MissionGen_C|GetHVTRemaining (Utilities|Array|Get(acopy) _outactors))
            (:%20%20
              _))
          (else
            (Math|Integer|DecrementInt (Variables|/Game/ReadyOrSwat/BluePrint/Tasks/MissionGen.MissionGen_C|GetTerryRemaining (Utilities|Array|Get(acopy) _outactors))
              (:%20%20
                _))))
        (Math|Integer|IncrementInt (Variables|/Game/ReadyOrSwat/BluePrint/RoS_Player.RoS_Player_C|GetPlayerPacified (Variables|Default|GetPlayerReferance))
          (:%20%20
            (return))))))
  (return))

(fn AiAimSkill
  (if (< (Variables|Default|GetAiSkill) 34)
    (return 45.0)
    (elif (< (Variables|Default|GetAiSkill) 67)
      (return 2e+01)
      (else
        (if (> (Variables|Default|GetAiSkill) 66)
          _
          (else
            _))
        (return 5.0)))))

(fn BulletSpawnTransform
  (bind _arrow1 (Variables|Default|GetArrow1))
  (bind _returnvalue (Transformation|GetWorldTransform _arrow1))
  (return (Math|Transform|MakeTransform (.location _returnvalue) (Math|Rotator|MakeRotfromX (Math|Random|RandomUnitVectorinConeinDegrees (Math|Vector|GetForwardVector (Pawn|GetControlRotation :!class /Script/Engine.Pawn)) (CallFunction|AiAimSkill))) (.scale _returnvalue))))

(fn AISkillBulletFear
  (if (< (Variables|Default|GetAiSkill) 34)
    (return 5.0)
    (elif (< (Variables|Default|GetAiSkill) 67)
      (return 2.5)
      (else
        (if (> (Variables|Default|GetAiSkill) 66)
          _
          (else
            _))
        (return 1.0)))))

(fn ShotLineTrace
  (bind _returnvalue (Transformation|GetActorLocation))
  (bind _outhit (Collision|LineTraceForObjects _returnvalue (+ _returnvalue (* (Math|Vector|GetForwardVector (Transformation|GetWorldRotation (Variables|Default|GetArrow1))) 5e+02)) (Utilities|Array|MakeArray "ObjectTypeQuery1" "ObjectTypeQuery2" "ObjectTypeQuery3" "ObjectTypeQuery6") false 0 "ForDuration"))
  (return _outhit))

(fn FrontFiringAcr
  (return (and (< (Math|Float|Absolute(Float) (.Yaw (Math|Rotator|BreakRotator (Math|Rotator|Delta(Rotator) (Math|Rotator|FindLookatRotation (Transformation|GetActorLocation) (Transformation|GetActorLocation (Variables|Default|GetPlayerReferance))) (Transformation|GetActorRotation))))) 9e+01) (< (Math|Vector|Distance(Vector) (Transformation|GetActorLocation) (Transformation|GetActorLocation (Variables|Default|GetPlayerReferance))) 7.5e+02))))
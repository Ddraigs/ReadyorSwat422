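; Behavior tree task for the Terrance AI that decides whether cover counts as valid, based on how far the AI is from the player.
; It reads the player actor from the blackboard and measures its distance to the controlled pawn, not to any cover point.
; It sets the CoverIsValid key true when that distance exceeds MinDistanceAwayFromPlayer, then always finishes successfully.
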(event EventReceiveExecuteAI
  (params (OwnerController :type AI%20Controller%20Object%20Reference) (ControlledPawn :type Pawn%20Object%20Reference))
  (Variables|Default|SetPlayerCharLoc (Transformation|GetActorLocation (AI|BehaviorTree|GetBlackboardValueasActor (Variables|Default|GetBB_PlayerReferance))))
  (Class|BTFunctionLibrary|SetBlackboardValueasBool (Variables|Default|GetCoverIsValid) (> (Math|Vector|VectorLength (- (Transformation|GetActorLocation ControlledPawn) (Variables|Default|GetPlayerCharLoc))) (Variables|Default|GetMinDistanceAwayFromPlayer)))
  (AI|BehaviorTree|FinishExecute true))
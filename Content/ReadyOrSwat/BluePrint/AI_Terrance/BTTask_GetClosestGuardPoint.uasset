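; Behavior tree task that picks the nearest free AI_GuardPoint for the controlled pawn to move to.
; It scans all guard points, shrinking DistanceTo as closer untaken ones appear and writing their location to the BBMoveLoc blackboard key.
; Taken points clear FoundPoint, even after an earlier match.
; If FoundPoint ends true the task succeeds; otherwise it writes the pawn's own location without calling FinishExecute.
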(event EventReceiveExecuteAI
  (params (OwnerController :type AI%20Controller%20Object%20Reference) (ControlledPawn :type Pawn%20Object%20Reference))
  (bind _outactors (Actor|GetAllActorsOfClass "/Game/ReadyOrSwat/BluePrint/AI/AI_GuardPoint.AI_GuardPoint_C"))
  (for _array_element _outactors
    (if (Variables|/Game/ReadyOrSwat/BluePrint/AI/AI_GuardPoint.AI_GuardPoint_C|GetIsTaken? _array_element)
      (Variables|Default|SetFoundPoint false)
      (elif (<= (Transformation|GetDistanceTo ControlledPawn _array_element) (Variables|Default|GetDistanceTo))
        (Variables|Default|SetDistanceTo (Transformation|GetDistanceTo ControlledPawn _array_element))
        (AI|BehaviorTree|SetBlackboardValueasVector (Variables|Default|GetBBMoveLoc) (Transformation|GetActorLocation _array_element))
        (Variables|Default|SetFoundPoint true))))
  (if (Variables|Default|GetFoundPoint)
    (AI|BehaviorTree|FinishExecute true)
    (else
      (AI|BehaviorTree|SetBlackboardValueasVector (Variables|Default|GetBBMoveLoc) (Transformation|GetActorLocation ControlledPawn)))))
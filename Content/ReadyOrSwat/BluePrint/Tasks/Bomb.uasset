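; Timed bomb objective with an on-screen countdown that explodes and damages nearby destructible actors when its timeline ends.
; Diffuise runs a second timeline while a RoSChar is in the box, filling a progress widget; RestDiffuse or leaving the box resets it.
; A completed defuse stops the bomb timer and decrements BombsRemaining on MissionGen.
; The defense AI spawning logic is disconnected and never runs.
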(event OnComponentBeginOverlap(Box)
  (params (OverlappedComponent :type Primitive%20Component%20Object%20Reference) (OtherActor :type Actor%20Object%20Reference) (OtherComp :type Primitive%20Component%20Object%20Reference) (OtherBodyIndex :type Integer) (bFromSweep :type Boolean) (SweepResult :type Hit%20Result%20Structure%20%28by%20ref%29))
  (bind _asro_schar (Utilities|Casting|CastToRoSChar OtherActor))
  (Variables|Default|SetCharRef _asro_schar))

(event OnComponentEndOverlap(Box)
  (params (OverlappedComponent :type Primitive%20Component%20Object%20Reference) (OtherActor :type Actor%20Object%20Reference) (OtherComp :type Primitive%20Component%20Object%20Reference) (OtherBodyIndex :type Integer))
  (bind _returnvalue (Transformation|GetActorLocation))
  (Variables|Default|SetCharRef 0)
  (Variables|/Game/ReadyOrSwat/UI/PlayerInterface/ProgressCounter.ProgressCounter_C|SetCountDown (Variables|Default|GetprogressCounter) 0.0)
  (bind _timeleft (Timeline|Diffuse Stop)
    (:Update
      (Variables|/Game/ReadyOrSwat/UI/PlayerInterface/ProgressCounter.ProgressCounter_C|SetCountDown (Variables|Default|GetprogressCounter) _timeleft))
    (:Finished
      (Variables|Default|SetDiffused true)
      (bind _outactors (Actor|GetAllActorsOfClass "/Game/ReadyOrSwat/BluePrint/Tasks/MissionGen.MissionGen_C"))
      (Math|Integer|DecrementInt (Variables|/Game/ReadyOrSwat/BluePrint/Tasks/MissionGen.MissionGen_C|GetBombsRemaining (Utilities|Array|Get(acopy) _outactors))
        (:%20%20
          (bind _countdown (Timeline|BombTimer Stop)
            (:Update
              (Variables|/Game/ReadyOrSwat/UI/PlayerInterface/CountDown.CountDown_C|SetCountDown (Variables|Default|GetCounter) _countdown))
            (:Finished
              (Effects|SpawnEmitteratLocation "/Game/StarterContent/Particles/P_Explosion.P_Explosion" (Transformation|GetActorLocation) "0, 0, 0" "50.000000,50.000000,50.000000")
              (bind _outhits (Collision|MultiSphereTraceForObjects _returnvalue _returnvalue 1.5e+03 (Utilities|Array|MakeArray "ObjectTypeQuery7") false 0 "ForDuration"))
              (for _array_element _outhits
                (bind _asdestructible_actor (Utilities|Casting|CastToDestructibleActor (.HitActor (Collision|BreakHitResult _array_element))))
                (Class|DestructibleComponent|ApplyRadiusDamage (Variables|/Script/ApexDestruction.DestructibleActor|GetDestructibleComponent _asdestructible_actor) 2e+04 (.Location (Collision|BreakHitResult _array_element)) 1.5e+03 2e+03 true)))))))))

(event Custom|RestDiffuse
  (bind _returnvalue (Transformation|GetActorLocation))
  (Variables|/Game/ReadyOrSwat/UI/PlayerInterface/ProgressCounter.ProgressCounter_C|SetCountDown (Variables|Default|GetprogressCounter) 0.0)
  (bind _timeleft (Timeline|Diffuse Stop)
    (:Update
      (Variables|/Game/ReadyOrSwat/UI/PlayerInterface/ProgressCounter.ProgressCounter_C|SetCountDown (Variables|Default|GetprogressCounter) _timeleft))
    (:Finished
      (Variables|Default|SetDiffused true)
      (bind _outactors (Actor|GetAllActorsOfClass "/Game/ReadyOrSwat/BluePrint/Tasks/MissionGen.MissionGen_C"))
      (Math|Integer|DecrementInt (Variables|/Game/ReadyOrSwat/BluePrint/Tasks/MissionGen.MissionGen_C|GetBombsRemaining (Utilities|Array|Get(acopy) _outactors))
        (:%20%20
          (bind _countdown (Timeline|BombTimer Stop)
            (:Update
              (Variables|/Game/ReadyOrSwat/UI/PlayerInterface/CountDown.CountDown_C|SetCountDown (Variables|Default|GetCounter) _countdown))
            (:Finished
              (Effects|SpawnEmitteratLocation "/Game/StarterContent/Particles/P_Explosion.P_Explosion" (Transformation|GetActorLocation) "0, 0, 0" "50.000000,50.000000,50.000000")
              (bind _outhits (Collision|MultiSphereTraceForObjects _returnvalue _returnvalue 1.5e+03 (Utilities|Array|MakeArray "ObjectTypeQuery7") false 0 "ForDuration"))
              (for _array_element _outhits
                (bind _asdestructible_actor (Utilities|Casting|CastToDestructibleActor (.HitActor (Collision|BreakHitResult _array_element))))
                (Class|DestructibleComponent|ApplyRadiusDamage (Variables|/Script/ApexDestruction.DestructibleActor|GetDestructibleComponent _asdestructible_actor) 2e+04 (.Location (Collision|BreakHitResult _array_element)) 1.5e+03 2e+03 true)))))))))

(event Custom|Diffuise
  (bind _returnvalue (Transformation|GetActorLocation))
  (Utilities|IsValid (Variables|Default|GetCharRef)
    (:Is%20Valid
      (bind _timeleft (Timeline|Diffuse PlayFromStart)
        (:Update
          (Variables|/Game/ReadyOrSwat/UI/PlayerInterface/ProgressCounter.ProgressCounter_C|SetCountDown (Variables|Default|GetprogressCounter) _timeleft))
        (:Finished
          (Variables|Default|SetDiffused true)
          (bind _outactors (Actor|GetAllActorsOfClass "/Game/ReadyOrSwat/BluePrint/Tasks/MissionGen.MissionGen_C"))
          (Math|Integer|DecrementInt (Variables|/Game/ReadyOrSwat/BluePrint/Tasks/MissionGen.MissionGen_C|GetBombsRemaining (Utilities|Array|Get(acopy) _outactors))
            (:%20%20
              (bind _countdown (Timeline|BombTimer Stop)
                (:Update
                  (Variables|/Game/ReadyOrSwat/UI/PlayerInterface/CountDown.CountDown_C|SetCountDown (Variables|Default|GetCounter) _countdown))
                (:Finished
                  (Effects|SpawnEmitteratLocation "/Game/StarterContent/Particles/P_Explosion.P_Explosion" (Transformation|GetActorLocation) "0, 0, 0" "50.000000,50.000000,50.000000")
                  (bind _outhits (Collision|MultiSphereTraceForObjects _returnvalue _returnvalue 1.5e+03 (Utilities|Array|MakeArray "ObjectTypeQuery7") false 0 "ForDuration"))
                  (for _array_element _outhits
                    (bind _asdestructible_actor (Utilities|Casting|CastToDestructibleActor (.HitActor (Collision|BreakHitResult _array_element))))
                    (Class|DestructibleComponent|ApplyRadiusDamage (Variables|/Script/ApexDestruction.DestructibleActor|GetDestructibleComponent _asdestructible_actor) 2e+04 (.Location (Collision|BreakHitResult _array_element)) 1.5e+03 2e+03 true)))))))))))

(event EventBeginPlay
  (bind _returnvalue (Transformation|GetActorLocation))
  (Utilities|FlowControl|Delay 0.2)
  (bind _returnvalue_2 (UserInterface|CreateWidget "/Game/ReadyOrSwat/UI/PlayerInterface/ProgressCounter.ProgressCounter_C"))
  (bind _output_get (Variables|Default|SetprogressCounter _returnvalue_2))
  (UserInterface|SetWidget (Variables|Default|GetWidget) _output_get)
  (bind _returnvalue_3 (UserInterface|CreateWidget "/Game/ReadyOrSwat/UI/PlayerInterface/CountDown.CountDown_C"))
  (bind _output_get_2 (Variables|Default|SetCounter _returnvalue_3))
  (UserInterface|Viewport|AddtoViewport _output_get_2 0)
  (bind _countdown (Timeline|BombTimer PlayFromStart)
    (:Update
      (Variables|/Game/ReadyOrSwat/UI/PlayerInterface/CountDown.CountDown_C|SetCountDown (Variables|Default|GetCounter) _countdown))
    (:Finished
      (Effects|SpawnEmitteratLocation "/Game/StarterContent/Particles/P_Explosion.P_Explosion" (Transformation|GetActorLocation) "0, 0, 0" "50.000000,50.000000,50.000000")
      (bind _outhits (Collision|MultiSphereTraceForObjects _returnvalue _returnvalue 1.5e+03 (Utilities|Array|MakeArray "ObjectTypeQuery7") false 0 "ForDuration"))
      (for _array_element _outhits
        (bind _asdestructible_actor (Utilities|Casting|CastToDestructibleActor (.HitActor (Collision|BreakHitResult _array_element))))
        (Class|DestructibleComponent|ApplyRadiusDamage (Variables|/Script/ApexDestruction.DestructibleActor|GetDestructibleComponent _asdestructible_actor) 2e+04 (.Location (Collision|BreakHitResult _array_element)) 1.5e+03 2e+03 true)))))

(fn ConstructionScript)

(fn SpawnDefenseAi)
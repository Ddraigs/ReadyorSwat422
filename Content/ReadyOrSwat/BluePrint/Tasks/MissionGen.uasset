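; Mission generator actor that builds a random set of objectives and ends the mission when all are cleared.
; StartMissionGen reads enabled types and objective count from RoSGameInstance, then rolls each from terrorist hunt, HVT, hostage or bomb defusal.
; Objectives spawn squad managers, guarded targets or bombs at spawn actors; hostage only prints a debug string.
; A looping timer checks remaining counters, then shows the ending stats screen once.
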(event Custom|StartMissionGen
  (bind _returnvalue (Game|GetGameInstance))
  (bind _asro_sgame_instance (Utilities|Casting|CastToRoSGameInstance _returnvalue))
  (Utilities|FlowControl|Delay 1.0)
  (Variables|Default|SetGameInstance _asro_sgame_instance)
  (Variables|Default|SetGameMode (.AsReady%20or%20Swat%20Game%20Mode (Utilities|Casting|CastToReadyOrSwatGameMode (Game|GetGameMode))))
  (Variables|Default|SetMG_EH_Enabled (Variables|/Game/ReadyOrSwat/BluePrint/RoSGameInstance.RoSGameInstance_C|GetEH_Enabled? _asro_sgame_instance))
  (Variables|Default|SetMG_BD_Enabled (Variables|/Game/ReadyOrSwat/BluePrint/RoSGameInstance.RoSGameInstance_C|GetBD_Enabled? _asro_sgame_instance))
  (Variables|Default|SetMG_HVT_Enabled (Variables|/Game/ReadyOrSwat/BluePrint/RoSGameInstance.RoSGameInstance_C|GetHVT_Enabled? _asro_sgame_instance))
  (Variables|Default|SetMG_H_Enabled (Variables|/Game/ReadyOrSwat/BluePrint/RoSGameInstance.RoSGameInstance_C|GetH_Enabled? _asro_sgame_instance))
  (for _index (range 0 (- (Math|Float|Truncate (Variables|/Game/ReadyOrSwat/BluePrint/RoSGameInstance.RoSGameInstance_C|GetObjectiveAmount _asro_sgame_instance)) 1))
    (bind _gamemode (CallFunction|DerterminAvliableGamemodes))
    (switch Utilities|FlowControl|Switch|SwitchonE_GameMode _gamemode
      (:NewEnumerator0
        (CallFunction|TerrorHunt)
        (Variables|Default|SetEH_Active true))
      (:NewEnumerator1
        (CallFunction|HVT)
        (Variables|Default|SetHVT_Active true))
      (:NewEnumerator2
        (CallFunction|Hostages)
        (Variables|Default|SetH_Active true))
      (:NewEnumerator4
        (CallFunction|BombDiffusal)
        (Variables|Default|SetBD_Active true))))
  (Utilities|Time|SetTimerbyEvent (delegate Custom|TimerTick) 5.0 true))

(event Custom|TimerTick
  (CallFunction|ISEHSucces)
  (CallFunction|ISHSucces)
  (CallFunction|ISHVTSecces)
  (CallFunction|ISBDSecces)
  (if (Math|Boolean|ANDBoolean (Variables|Default|GetEH_Succes) (Variables|Default|GetH_Succes) (Variables|Default|GetHVT_Succes) (Variables|Default|GetBD_Succes))
    (CallFunction|Finish)))

(event Custom|Finish
  (Utilities|FlowControl|DoOnce false
    (:Completed
      (bind _returnvalue (UserInterface|CreateWidget "/Game/ReadyOrSwat/UI/PlayerInterface/PlayerEndingStatScreen.PlayerEndingStatScreen_C"))
      (UserInterface|Viewport|AddtoViewport _returnvalue 0))))

(event EventBeginPlay)

(fn ConstructionScript)

(fn SetupHoldoutPlayers
  (params (InputPin :type Ro%20S%20Player%20Object%20Reference))
  (bind _returnvalue (Utilities|GetDataTableRow "/Game/ReadyOrSwat/UI/DataTables/DataOfItems.DataOfItems" "M4")
    (:then
      (bind _output_get (Variables|/Game/ReadyOrSwat/BluePrint/RoSChar.RoSChar_C|SetPrimaryWeapon InputPin (.Weapon (Utilities|Struct|BreakS_Loadout _returnvalue))))
      (Variables|/Game/ReadyOrSwat/BluePrint/RoSChar.RoSChar_C|SetWeapon_Ref InputPin _output_get)
      (Variables|/Game/ReadyOrSwat/BluePrint/RoSChar.RoSChar_C|SetPrimaryAmmo InputPin (.Ammount (Utilities|Struct|BreakS_Loadout _returnvalue)))
      (bind _returnvalue_2 (Utilities|GetDataTableRow "/Game/ReadyOrSwat/UI/DataTables/DataOfItems.DataOfItems" "M9")
        (:then
          (Variables|/Game/ReadyOrSwat/BluePrint/RoSChar.RoSChar_C|SetSecondaryWeapon InputPin (.Weapon (Utilities|Struct|BreakS_Loadout _returnvalue_2)))
          (Variables|/Game/ReadyOrSwat/BluePrint/RoSChar.RoSChar_C|SetSecondaryAmmo InputPin (.Ammount (Utilities|Struct|BreakS_Loadout _returnvalue_2)))
          (Default|SetActivePlayerWeaponMesh InputPin))))))

(fn DerterminAvliableGamemodes
  (if (Variables|Default|GetMG_EH_Enabled)
    (if (> (Math|Random|RandomIntegerinRange 0 100) 33)
      (LocalVariables|SetLocalGameMode "NewEnumerator0")
      (else
        (if (Variables|Default|GetMG_H_Enabled) :!label _label
          (if (> (Math|Random|RandomIntegerinRange 0 100) 50)
            (LocalVariables|SetLocalGameMode "NewEnumerator2")
            (else
              (if (Variables|Default|GetMG_HVT_Enabled) :!label _label_2
                (if (> (Math|Random|RandomIntegerinRange 0 100) 50)
                  (LocalVariables|SetLocalGameMode "NewEnumerator1")
                  (else
                    (if (Variables|Default|GetMG_BD_Enabled) :!label _label_3
                      (if (> (Math|Random|RandomIntegerinRange 0 100) 50)
                        (LocalVariables|SetLocalGameMode "NewEnumerator4")
                        (else
                          (if (Variables|Default|GetMG_EH_Enabled) :!label _label_4
                            (LocalVariables|SetLocalGameMode "NewEnumerator0")
                            (elif (Variables|Default|GetMG_BD_Enabled)
                              (LocalVariables|SetLocalGameMode "NewEnumerator4")
                              (elif (Variables|Default|GetMG_HVT_Enabled)
                                (LocalVariables|SetLocalGameMode "NewEnumerator1")
                                (elif (Variables|Default|GetMG_H_Enabled)
                                  (LocalVariables|SetLocalGameMode "NewEnumerator2")
                                  (else
                                    (LocalVariables|SetLocalGameMode "NewEnumerator0"))))))))
                      (else
                        (goto _label_4)))))
                (else
                  (goto _label_3)))))
          (else
            (goto _label_2)))))
    (else
      (goto _label)))
  (return (LocalVariables|GetLocalGameMode)))

(fn TerrorHunt
  (bind _outactors (Actor|GetAllActorsOfClass "/Game/ReadyOrSwat/BluePrint/Tasks/SpawnPoint.SpawnPoint_C"))
  (bind (_array_element _array_index) (Utilities|Array|ForEachLoopwithBreak _outactors :!label _label)
    (:LoopBody
      (if (not (Variables|/Game/ReadyOrSwat/BluePrint/Tasks/SpawnPoint.SpawnPoint_C|GetUsed? _array_element))
        (Game|SpawnActorfromClass "/Game/ReadyOrSwat/BluePrint/AI_Terrance/SquadManager.SquadManager_C" (Transformation|GetActorTransform _array_element) "AlwaysSpawn" 0 7 _array_index (Variables|Default|GetGameMode) self 0)
        (Variables|/Game/ReadyOrSwat/BluePrint/Tasks/SpawnPoint.SpawnPoint_C|SetUsed? _array_element true)
        (goto _label Break)))
    (:Completed
      (return))))

(fn BombDiffusal
  (bind _outactors (Actor|GetAllActorsOfClass "/Game/ReadyOrSwat/BluePrint/Tasks/BombSpawn.BombSpawn_C"))
  (Game|SpawnActorfromClass "/Game/ReadyOrSwat/BluePrint/Tasks/Bomb.Bomb_C" (Transformation|GetActorTransform (Utilities|Array|Get(acopy) _outactors (Math|Random|RandomIntegerinRange 0 (Utilities|Array|LastIndex _outactors)))) "Undefined" 0 0)
  (Math|Integer|IncrementInt (Variables|Default|GetBombsRemaining)))

(fn HVT
  (bind _outactors (Actor|GetAllActorsOfClass "/Game/ReadyOrSwat/BluePrint/Tasks/HVTSpawn.HVTSpawn_C"))
  (Game|SpawnActorfromClass "/Game/ReadyOrSwat/BluePrint/AI/AI_Char_Terry.AI_Char_Terry_C" (Transformation|GetActorTransform (Utilities|Array|Get(acopy) _outactors (Math|Random|RandomIntegerinRange 0 (Utilities|Array|LastIndex _outactors)))) "AlwaysSpawn" 0 75 "NewEnumerator1" true 0)
  (Math|Integer|IncrementInt (Variables|Default|GetHVTRemaining)
    (:%20%20
      (for _index (range 0 3)
        (Game|SpawnActorfromClass "/Game/ReadyOrSwat/BluePrint/AI/AI_Char_Terry.AI_Char_Terry_C" (Math|Transform|MakeTransform (Math|Vector|MakeVector (.x (Math|Random|RandomPointinBoundingBox (Transformation|GetActorLocation (Utilities|Array|Get(acopy) _outactors (Math|Random|RandomIntegerinRange 0 (Utilities|Array|LastIndex _outactors)))) (Components|Box|GetScaledBoxExtent (Variables|/Game/ReadyOrSwat/BluePrint/Tasks/HVTSpawn.HVTSpawn_C|GetBox (Utilities|Array|Get(acopy) _outactors (Math|Random|RandomIntegerinRange 0 (Utilities|Array|LastIndex _outactors))))))) (.y (Math|Random|RandomPointinBoundingBox (Transformation|GetActorLocation (Utilities|Array|Get(acopy) _outactors (Math|Random|RandomIntegerinRange 0 (Utilities|Array|LastIndex _outactors)))) (Components|Box|GetScaledBoxExtent (Variables|/Game/ReadyOrSwat/BluePrint/Tasks/HVTSpawn.HVTSpawn_C|GetBox (Utilities|Array|Get(acopy) _outactors (Math|Random|RandomIntegerinRange 0 (Utilities|Array|LastIndex _outactors))))))) (.Z (Math|Vector|BreakVector (Transformation|GetActorLocation (Utilities|Array|Get(acopy) _outactors (Math|Random|RandomIntegerinRange 0 (Utilities|Array|LastIndex _outactors)))))))) "AdjustIfPossibleButDontSpawnIfColliding" 0 (Math|Random|RandomIntegerinRange 0 33) "NewEnumerator0" false 0))
      (for _index_2 (range 0 2)
        (Game|SpawnActorfromClass "/Game/ReadyOrSwat/BluePrint/AI/AI_Char_Terry.AI_Char_Terry_C" (Math|Transform|MakeTransform (Math|Vector|MakeVector (.x (Math|Random|RandomPointinBoundingBox (Transformation|GetActorLocation (Utilities|Array|Get(acopy) _outactors (Math|Random|RandomIntegerinRange 0 (Utilities|Array|LastIndex _outactors)))) (Components|Box|GetScaledBoxExtent (Variables|/Game/ReadyOrSwat/BluePrint/Tasks/HVTSpawn.HVTSpawn_C|GetBox (Utilities|Array|Get(acopy) _outactors (Math|Random|RandomIntegerinRange 0 (Utilities|Array|LastIndex _outactors))))))) (.y (Math|Random|RandomPointinBoundingBox (Transformation|GetActorLocation (Utilities|Array|Get(acopy) _outactors (Math|Random|RandomIntegerinRange 0 (Utilities|Array|LastIndex _outactors)))) (Components|Box|GetScaledBoxExtent (Variables|/Game/ReadyOrSwat/BluePrint/Tasks/HVTSpawn.HVTSpawn_C|GetBox (Utilities|Array|Get(acopy) _outactors (Math|Random|RandomIntegerinRange 0 (Utilities|Array|LastIndex _outactors))))))) (.Z (Math|Vector|BreakVector (Transformation|GetActorLocation (Utilities|Array|Get(acopy) _outactors (Math|Random|RandomIntegerinRange 0 (Utilities|Array|LastIndex _outactors)))))))) "AdjustIfPossibleButDontSpawnIfColliding" 0 (Math|Random|RandomIntegerinRange 34 67) "NewEnumerator0" false 0)))))

(fn Hostages
  (Development|PrintString "I AM HOSTAGE!"))

(fn CreateSqaud
  (params (SpawnPoint :type Spawn%20Point%20Object%20Reference))
  (Game|SpawnActorfromClass "/Game/ReadyOrSwat/BluePrint/AI/AI_Char_Terry.AI_Char_Terry_C" (CallFunction|SpawnWithinExtend SpawnPoint) "AlwaysSpawn" 0 (Math|Random|RandomIntegerinRange 68 100) "NewEnumerator0" false 0)
  (Math|Integer|IncrementInt (Variables|Default|GetTerryRemaining)
    (:%20%20
      (for _index (range 0 3)
        (Game|SpawnActorfromClass "/Game/ReadyOrSwat/BluePrint/AI/AI_Char_Terry.AI_Char_Terry_C" (CallFunction|SpawnWithinExtend SpawnPoint) "AdjustIfPossibleButAlwaysSpawn" 0 (Math|Random|RandomIntegerinRange 0 33) "NewEnumerator0" false 0)
        (Math|Integer|IncrementInt (Variables|Default|GetTerryRemaining)))
      (for _index_2 (range 0 2)
        (Game|SpawnActorfromClass "/Game/ReadyOrSwat/BluePrint/AI/AI_Char_Terry.AI_Char_Terry_C" (CallFunction|SpawnWithinExtend SpawnPoint) "AdjustIfPossibleButAlwaysSpawn" 0 (Math|Random|RandomIntegerinRange 34 67) "NewEnumerator0" false 0)
        (Math|Integer|IncrementInt (Variables|Default|GetTerryRemaining)))
      (return))))

(fn SpawnWithinExtend
  (params (self2 :type Spawn%20Point%20Object%20Reference))
  (bind _returnvalue (Transformation|GetActorLocation self2))
  (bind _box (Variables|/Game/ReadyOrSwat/BluePrint/Tasks/SpawnPoint.SpawnPoint_C|GetBox self2))
  (bind _returnvalue_2 (Components|Box|GetScaledBoxExtent _box))
  (bind _returnvalue_3 (Math|Random|RandomPointinBoundingBox _returnvalue _returnvalue_2))
  (return (Math|Transform|MakeTransform (Math|Vector|MakeVector (.x _returnvalue_3) (.y _returnvalue_3) (.Z (Math|Vector|BreakVector _returnvalue))))))

(fn ISEHSucces
  (if (Variables|Default|GetEH_Active)
    (if (< (Variables|Default|GetTerryRemaining) 1)
      (Variables|Default|SetEH_Succes true)
      (else
        (Variables|Default|SetEH_Succes false)))
    (else
      (Variables|Default|SetEH_Succes true)))
  (return))

(fn ISHSucces
  (if (Variables|Default|GetH_Active)
    (if (== (Variables|Default|GetHostagesRemaining) 0)
      (Variables|Default|SetH_Succes true)
      (else
        (Variables|Default|SetH_Succes false)))
    (else
      (Variables|Default|SetH_Succes true)))
  (return))

(fn ISHVTSecces
  (if (Variables|Default|GetHVT_Active)
    (if (== (Variables|Default|GetHVTRemaining) 0)
      (Variables|Default|SetHVT_Succes true)
      (else
        (Variables|Default|SetHVT_Succes false)))
    (else
      (Variables|Default|SetHVT_Succes true)))
  (return))

(fn ISBDSecces
  (if (Variables|Default|GetBD_Active)
    (if (== (Variables|Default|GetBombsRemaining) 0)
      (Variables|Default|SetBD_Succes true)
      (else
        (Variables|Default|SetBD_Succes false)))
    (else
      (Variables|Default|SetBD_Succes true)))
  (return))
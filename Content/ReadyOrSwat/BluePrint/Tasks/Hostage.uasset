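; Hostage character Blueprint that players free by holding a timed rescue, which counts toward the mission's remaining hostages.
; A timeline fills a ProgressCounter widget, guarded by a DoOnce so repeated Rescued calls don't restart it.
; On completion it decrements MissionGenSysRef.HostagesRemaining, sends the AI controller to the first Safepoint found and destroys itself after a delay.
; Stop cancels an unfinished rescue, resetting the counter and hiding the widget.
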(event Custom|Rescued
  (Utilities|FlowControl|DoOnce false
    (:Completed
      (Rendering|SetVisibility (Variables|Default|GetWidget) true false)
      (bind _newtrack_0 (Timeline|Timeline_0 PlayFromStart)
        (:Update
          (Variables|/Game/ReadyOrSwat/UI/PlayerInterface/ProgressCounter.ProgressCounter_C|SetCountDown (Variables|Default|GetProgressCounter) _newtrack_0))
        (:Finished
          (Math|Integer|DecrementInt (Variables|/Game/ReadyOrSwat/BluePrint/Tasks/MissionGen.MissionGen_C|GetHostagesRemaining (Variables|Default|GetMissionGenSysRef))
            (:%20%20
              (Variables|Default|SetRescued? true)
              (Rendering|SetVisibility (Variables|Default|GetWidget) false false)
              (Development|PrintString "Saved")
              (AI|Navigation|MovetoActor (AI|GetAIController self) (Variables|Default|GetSafepoint) 5e+01 true true true 0)
              (Utilities|FlowControl|Delay 1e+01)
              (Actor|DestroyActor))))))))

(event Custom|Stop
  (if (not (Variables|Default|GetRescued?))
    (Utilities|FlowControl|Sequence
      (:then_0
        (bind _newtrack_0 (Timeline|Timeline_0 Stop)
          (:Update
            (Variables|/Game/ReadyOrSwat/UI/PlayerInterface/ProgressCounter.ProgressCounter_C|SetCountDown (Variables|Default|GetProgressCounter) _newtrack_0))
          (:Finished
            (Math|Integer|DecrementInt (Variables|/Game/ReadyOrSwat/BluePrint/Tasks/MissionGen.MissionGen_C|GetHostagesRemaining (Variables|Default|GetMissionGenSysRef))
              (:%20%20
                (Variables|Default|SetRescued? true)
                (Rendering|SetVisibility (Variables|Default|GetWidget) false false)
                (Development|PrintString "Saved")
                (AI|Navigation|MovetoActor (AI|GetAIController self) (Variables|Default|GetSafepoint) 5e+01 true true true 0)
                (Utilities|FlowControl|Delay 1e+01)
                (Actor|DestroyActor))))))
      (:then_1
        (Variables|/Game/ReadyOrSwat/UI/PlayerInterface/ProgressCounter.ProgressCounter_C|SetCountDown (Variables|Default|GetprogressCounter) 0.0)
        (Utilities|FlowControl|DoOnce false) ; enters at Reset
      )
      (:then_2
        (Utilities|FlowControl|Delay 0.5)
        (Rendering|SetVisibility (Variables|Default|GetWidget) false false)))))

(event EventBeginPlay
  (bind _returnvalue (UserInterface|CreateWidget "/Game/ReadyOrSwat/UI/PlayerInterface/ProgressCounter.ProgressCounter_C"))
  (bind _output_get (Variables|Default|SetprogressCounter _returnvalue))
  (UserInterface|SetWidget (Variables|Default|GetWidget) _output_get)
  (bind _outactors (Actor|GetAllActorsOfClass "/Game/ReadyOrSwat/BluePrint/Tasks/Safepoint.Safepoint_C"))
  (Variables|Default|SetSafepoint (Utilities|Array|Get(acopy) _outactors)))

(fn ConstructionScript)
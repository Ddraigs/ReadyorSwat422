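; Holdout game mode that runs waves of Terry AI enemies and shows an ending screen once all players are dead.
; WaveCheck detects an empty enemy array, spawns restock boxes and runs a timeline intermission before WaveSpawn removes them.
; WaveSpawn places enemies randomly within the first HoldSpawnPoints box, with count and health from per-wave curves.
; BeginPlay is empty, leaving the WaveCheck timer and wave counter setup disconnected.
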(event Custom|WaveSpawn
  (bind _aihealthcurve (Variables|Default|GetAIHealthCurve))
  (bind _waves (Variables|Default|GetWaves))
  (bind _returnvalue (Math|Conversions|ToFloat(Integer) _waves))
  (bind _returnvalue_2 (Math|Curves|GetFloatValue _aihealthcurve _returnvalue))
  (Variables|Default|SetWaveInprogress true)
  (for _array_element (Variables|Default|GetRestockBox)
    (Default|CloseMenu _array_element)
    (Actor|DestroyActor _array_element))
  (bind _outactors (Actor|GetAllActorsOfClass "/Game/ReadyOrSwat/BluePrint/Tasks/HoldSpawnPoints.HoldSpawnPoints_C"))
  (Variables|Default|SetSpawnbox (Utilities|Array|Get(acopy) _outactors))
  (for _index (range 0 (Math|Float|Truncate (Math|Curves|GetFloatValue (Variables|Default|GetWaveSpawnCurve) (Math|Conversions|ToFloat(Integer) (Variables|Default|GetWaves)))))
    (bind _returnvalue_3 (AI|SpawnAIFromClass "/Game/ReadyOrSwat/BluePrint/AI/AI_Char_Terry.AI_Char_Terry_C" "/Game/ReadyOrSwat/BluePrint/AI/BT_AI_Terry.BT_AI_Terry" (Math|Vector|MakeVector (.x (Math|Random|RandomPointinBoundingBox (.Origin (Collision|GetComponentBounds (Variables|/Game/ReadyOrSwat/BluePrint/Tasks/HoldSpawnPoints.HoldSpawnPoints_C|GetBox (Variables|Default|GetSpawnbox)))) (.BoxExtent (Collision|GetComponentBounds (Variables|/Game/ReadyOrSwat/BluePrint/Tasks/HoldSpawnPoints.HoldSpawnPoints_C|GetBox (Variables|Default|GetSpawnbox)))))) (.y (Math|Random|RandomPointinBoundingBox (.Origin (Collision|GetComponentBounds (Variables|/Game/ReadyOrSwat/BluePrint/Tasks/HoldSpawnPoints.HoldSpawnPoints_C|GetBox (Variables|Default|GetSpawnbox)))) (.BoxExtent (Collision|GetComponentBounds (Variables|/Game/ReadyOrSwat/BluePrint/Tasks/HoldSpawnPoints.HoldSpawnPoints_C|GetBox (Variables|Default|GetSpawnbox)))))) (.z (Math|Random|RandomPointinBoundingBox (.Origin (Collision|GetComponentBounds (Variables|/Game/ReadyOrSwat/BluePrint/Tasks/HoldSpawnPoints.HoldSpawnPoints_C|GetBox (Variables|Default|GetSpawnbox)))) (.BoxExtent (Collision|GetComponentBounds (Variables|/Game/ReadyOrSwat/BluePrint/Tasks/HoldSpawnPoints.HoldSpawnPoints_C|GetBox (Variables|Default|GetSpawnbox))))))) "0, 0, 0" true))
    (bind _asai_char_terry (Utilities|Casting|CastToAI_Char_Terry _returnvalue_3))
    (Variables|/Game/ReadyOrSwat/BluePrint/AI/AI_Char_Terry.AI_Char_Terry_C|SetAIType _asai_char_terry "NewEnumerator2")
    (Variables|/Game/ReadyOrSwat/BluePrint/AI/AI_Char_Terry.AI_Char_Terry_C|SetHealth _asai_char_terry _returnvalue_2)
    (Variables|/Game/ReadyOrSwat/BluePrint/AI/AI_Char_Terry.AI_Char_Terry_C|SetHealthMax _asai_char_terry _returnvalue_2)
    (Utilities|Array|AddUnique (Variables|Default|GetTerryArray) _asai_char_terry)))

(event Custom|WaveCheck
  (if (Variables|Default|GetWaveInprogress)
    (bind _outactors (Actor|GetAllActorsOfClass "/Game/ReadyOrSwat/BluePrint/RoS_Player.RoS_Player_C"))
    (Variables|Default|SetHowmanyDead 0)
    (for _array_element _outactors
      (if (Variables|/Game/ReadyOrSwat/BluePrint/RoSChar.RoSChar_C|GetIsDead _array_element)
        (Math|Integer|IncrementInt (Variables|Default|GetHowmanyDead))))
    (if (not (>= (Variables|Default|GetHowmanyDead) (Utilities|Array|Length _outactors)))
      (if (< (Utilities|Array|LastIndex (Variables|Default|GetTerryArray)) 0)
        (Variables|Default|SetWaveInprogress false)
        (CallFunction|SpawnRestockBox)
        (Math|Integer|IncrementInt (Variables|Default|GetWaves)
          (:%20%20
            (bind _timeleft (Timeline|WaveIntermission PlayFromStart)
              (:Update
                (Variables|Default|SetTimeBetweenWaves _timeleft))
              (:Finished
                (CallFunction|WaveSpawn))))))
      (else
        (Viewport|RemoveAllWidgets)
        (bind _returnvalue (UserInterface|CreateWidget "/Game/ReadyOrSwat/UI/Menu/EndingScreen.EndingScreen_C"))
        (UserInterface|Viewport|AddtoViewport _returnvalue 0)))))

(event EventBeginPlay)

(fn ConstructionScript
  (|CallParentFunction)
  (Components|Box|SetBoxExtent (Variables|Default|GetSpawn_1) (Variables|Default|GetBoxExtent) true))

(fn SpawnRestockBox
  (bind _outactors (Actor|GetAllActorsOfClass "/Game/ReadyOrSwat/BluePrint/Tasks/RestockSpawnLoc.RestockSpawnLoc_C"))
  (for _array_element _outactors
    (bind _returnvalue (Game|SpawnActorfromClass "/Game/ReadyOrSwat/BluePrint/Interabtables/Restock.Restock_C" (Transformation|GetActorTransform _array_element) "Undefined" 0 "150.000000,50.000000,100.000000" 0))
    (Utilities|Array|AddUnique (Variables|Default|GetRestockBox) _returnvalue))
  (return))